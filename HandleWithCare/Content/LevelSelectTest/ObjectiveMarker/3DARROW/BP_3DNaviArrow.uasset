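; BP_3DNaviArrow is a 3D navigation arrow that points in the direction of an objective from the player.
; On BeginPlay it finds a Temp_Tracker actor and caches its location once, so later movement of that actor is not followed.
; Each Tick it computes the look-at rotation from the player pawn to that location and applies only the yaw to ArrowMesh, keeping the arrow level.
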(event `self.ReceiveBeginPlay`
  (bind _returnvalue (`GameplayStatics.GetActorOfClass` "/Game/LevelSelectTest/ObjectiveMarker/Temp_Tracker.Temp_Tracker_C"))
  (set `self.TargetObjective` (`self.K2_GetActorLocation` _returnvalue)))

(event `self.ReceiveTick`
  (params (DeltaSeconds :type "Float (single-precision)"))
  (bind (_returnvalue_roll _returnvalue_pitch _returnvalue_yaw) (`KismetMathLibrary.BreakRotator` (`KismetMathLibrary.FindLookAtRotation` (`SceneComponent.K2_GetComponentLocation` (`Actor.RootComponent` (`GameplayStatics.GetPlayerPawn` 0))) (`self.TargetObjective`))))
  (`SceneComponent.K2_SetWorldRotation` (`self.ArrowMesh`) (`KismetMathLibrary.MakeRotator` 0.0 0.0 _returnvalue_yaw) false false))

(fn `UserConstructionScript`)