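; Player character for a level-select test that brings up a level confirmation widget.
; BeginPlay creates the BP_LevelConfrimWidget and shows the mouse cursor, and pressing E adds the widget to the viewport without checking for overlap.
; Mesh overlap sets an Overlapping flag that is never cleared; the branch that would use it to open ThirdPersonMap is disconnected and never runs.
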(event `self.Mesh.OnComponentBeginOverlap`
  (params (OverlappedComponent :type "PrimitiveComponent Object Reference") (OtherActor :type "Actor Object Reference") (OtherComp :type "PrimitiveComponent Object Reference") (OtherBodyIndex :type Integer) (bFromSweep :type Boolean) (SweepResult :type "HitResult Structure (by ref)"))
  (set `self.overlapping` true))

(event `Key|E`
  (params (Key :type "Key Structure"))
  (:`Pressed`
    (`UserWidget.AddToViewport` (`self.ConfirmWidget`) 0)))

(event `self.ReceiveBeginPlay`
  (`GameplayStatics.GetActorOfClass` (`GameplayStatics.GetObjectClass` (stale `self.Mesh.OnComponentBeginOverlap` OtherActor)))
  (bind _returnvalue (`|CreateWidget` "/Game/LevelSelectTest/Widgets/BP_LevelConfrimWidget.BP_LevelConfrimWidget_C"))
  (set `self.ConfirmWidget` _returnvalue)
  (set `PlayerController.bShowMouseCursor` true (`GameplayStatics.GetPlayerController` 0)))

(fn `UserConstructionScript`)