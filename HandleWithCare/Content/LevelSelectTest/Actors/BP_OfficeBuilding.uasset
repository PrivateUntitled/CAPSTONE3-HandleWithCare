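; BP_OfficeBuilding is a level actor for an office building that can serve as the quest objective for the player's truck.
; On BeginPlay, if the game instance's current objective matches one specific enum entry, it sets its quest trigger to that entry.
; It then sets the vehicle truck's target objective to its own location.
; The construction script only calls the parent implementation.
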(event `self.ReceiveBeginPlay`
  (`parent.ReceiveBeginPlay`)
  (if (`|EnumEquality` (`/Game/GameInstance/BP_GameInstance.CurrentObjective` (`self.As BP Game Instance`)) "NewEnumerator12")
    (set `self.QuestTrigger` "NewEnumerator12")
    (set `/Game/Blueprints/CarMovement/BP_Vehicle_Truck.TargetObjective` (`self.K2_GetActorLocation`) (`self.As BP Vehicle Truck`))))

(fn `UserConstructionScript`
  (`parent.UserConstructionScript`))