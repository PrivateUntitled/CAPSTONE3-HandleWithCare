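; BP_AC_PickUp lets the player pick up the currently hovered item with the E key.
; On BeginPlay it caches the player's BP_ThirdPersonCharacter, then on E reads that character's CurrentHoveredItem.
; The item attaches to the character's SMAssetPlatform, snaps to its world location, is stored as CurrentHeldItem and has its mesh collision disabled.
; It also prints the item's name; no drop logic is present.
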(event `self.ReceiveBeginPlay`
  (bind _asbp_third_person_character (cast `/Game/ThirdPerson/Blueprints/BP_ThirdPersonCharacter` (`GameplayStatics.GetPlayerPawn` 0)))
  (set `self.As BP Third Person Character` _asbp_third_person_character))

(event `Key|E`
  (params (Key :type "Key Structure"))
  (bind _as_bp_third_person_character (`self.As BP Third Person Character`))
  (bind _currenthovereditem (`/Game/ThirdPerson/Blueprints/BP_ThirdPersonCharacter.CurrentHoveredItem` _as_bp_third_person_character))
  (bind _sm_assetplatform (`/Game/ThirdPerson/Blueprints/BP_ThirdPersonCharacter.SM_AssetPlatform` _as_bp_third_person_character))
  (:`Pressed`
    (if (not (== _currenthovereditem null))
      (`KismetSystemLibrary.PrintString` (`KismetSystemLibrary.GetDisplayName` _currenthovereditem))
      (`Actor.K2_AttachToComponent` _currenthovereditem _sm_assetplatform "None" "KeepWorld" "KeepWorld" "KeepWorld" true)
      (`Actor.K2_SetActorLocation` _currenthovereditem (`SceneComponent.K2_GetComponentLocation` _sm_assetplatform) false false)
      (bind _output_get (set `self.CurrentHeldItem` _currenthovereditem))
      (`PrimitiveComponent.SetCollisionEnabled` (`/Game/Blueprints/ItemInteractables/BP_A_ItemInteractable.StaticMesh` _output_get) "NoCollision"))))