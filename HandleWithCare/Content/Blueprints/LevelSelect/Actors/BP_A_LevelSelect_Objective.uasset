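; Level-select objective actor that completes a truck destination and hands the player on to the office building.
; On BeginPlay it points the truck's target at its trigger box when the GameInstance objective matches.
; Overlapping the box then clears sequencer dialogue and teleports the truck to its mesh under a camera fade.
; It then updates the objective, office quest trigger and truck target, and queues Level 1 end dialogue.
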(event `self.ReceiveBeginPlay`
  (bind _asbp_game_instance (cast `/Game/GameInstance/BP_GameInstance` (`GameplayStatics.GetGameInstance`)))
  (set `self.As BP Game Instance` _asbp_game_instance)
  (bind _asbp_truck_ls (cast `/Game/Blueprints/CarMovement/BP_TruckLS` (`GameplayStatics.GetPlayerPawn` 0)))
  (set `self.As BP Truck LS` _asbp_truck_ls)
  (if (`|EnumEquality` (`/Game/GameInstance/BP_GameInstance.CurrentObjective` (`self.As BP Game Instance`)) "NewEnumerator10")
    (set `/Game/Blueprints/CarMovement/BP_TruckLS.TargetObjective` (`SceneComponent.K2_GetComponentLocation` (`self.Box`)) (`self.As BP Truck LS`))))

(event `StartFade`
  (bind _as_bp_truck_ls (`self.As BP Truck LS`))
  (bind _returnvalue (`GameplayStatics.GetActorOfClass` "/Game/Blueprints/Narrative/BP_LevelSelect_Sequencer.BP_LevelSelect_Sequencer_C"))
  (bind _narrative (`/Game/Blueprints/Narrative/AC_Narrative.Narrative` (`/Game/Blueprints/Narrative/BP_LevelSequencer.AC_Narrative` _returnvalue)))
  (`KismetArrayLibrary.Array_Clear` (`/Game/Blueprints/Narrative/WB_Narrative.DialogueBlock` _narrative))
  (`PanelWidget.ClearChildren` (`/Game/Blueprints/Narrative/WB_Narrative.NarrativeBlockContainer` _narrative))
  (`PlayerCameraManager.StartCameraFade` :`self` (`GameplayStatics.GetPlayerCameraManager` 0) :`ToAlpha` 1.0 :`Duration` 2.0 :`bHoldWhenFinished` true)
  (`KismetSystemLibrary.Delay` 2.0)
  (`self.K2_SetActorLocation` _as_bp_truck_ls (`SceneComponent.K2_GetComponentLocation` (`self.StaticMesh`)) false false)
  (`self.K2_SetActorRotation` :`self` _as_bp_truck_ls)
  (`KismetSystemLibrary.Delay` 1.0)
  (`PlayerCameraManager.StartCameraFade` :`self` (`GameplayStatics.GetPlayerCameraManager` 0) :`FromAlpha` 1.0 :`Duration` 2.0 :`bHoldWhenFinished` true)
  (set `/Game/GameInstance/BP_GameInstance.CurrentObjective` "NewEnumerator9" (`self.As BP Game Instance`))
  (bind _returnvalue_2 (`GameplayStatics.GetActorOfClass` "/Game/Blueprints/LevelSelect/Actors/BP_OfficeBuilding.BP_OfficeBuilding_C"))
  (set `/Game/Blueprints/LevelSelect/Actors/BP_BaseBuilding.QuestTrigger` "NewEnumerator9" _returnvalue_2)
  (set `/Game/Blueprints/CarMovement/BP_TruckLS.TargetObjective` (`self.K2_GetActorLocation` _returnvalue_2) (`self.As BP Truck LS`))
  (bind _returnvalue_3 (`GameplayStatics.GetActorOfClass` "/Game/Blueprints/Narrative/BP_LevelSelect_Sequencer.BP_LevelSelect_Sequencer_C"))
  (`/Game/Blueprints/Narrative/AC_Narrative.AddDialogue` (`/Game/Blueprints/Narrative/BP_LevelSequencer.AC_Narrative` _returnvalue_3) "/Game/Blueprints/Narrative/DataAssets/LevelSelect/LevelSelect_Level1/DA_DG_LevelSelect_Level1_End.DA_DG_LevelSelect_Level1_End"))

(event `self.Box.OnComponentBeginOverlap`
  (params (OverlappedComponent :type "PrimitiveComponent Object Reference") (OtherActor :type "Actor Object Reference") (OtherComp :type "PrimitiveComponent Object Reference") (OtherBodyIndex :type Integer) (bFromSweep :type Boolean) (SweepResult :type "HitResult Structure (by ref)"))
  (if (`|EnumEquality` (`/Game/GameInstance/BP_GameInstance.CurrentObjective` (`self.As BP Game Instance`)) "NewEnumerator10")
    (`self.StartFade`)))

(fn `UserConstructionScript`)