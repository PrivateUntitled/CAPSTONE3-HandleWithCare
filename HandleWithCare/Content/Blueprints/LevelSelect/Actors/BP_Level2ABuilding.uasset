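; BP_Level2ABuilding is a level select building actor that can set where the level select truck starts.
; On BeginPlay it runs the parent logic, then checks the game instance's current objective.
; If that objective matches one specific enum value, it moves BP_TruckLS to its SpawnLocation component's world position without sweeping.
; Overlap, Tick and the construction script add no logic of their own.
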(event `self.ReceiveBeginPlay`
  (`parent.ReceiveBeginPlay`)
  (if (`|EnumEquality` (`/Game/GameInstance/BP_GameInstance.CurrentObjective` (`self.As BP Game Instance`)) "NewEnumerator6")
    (`self.K2_SetActorLocation` (`self.As BP Truck LS`) (`SceneComponent.K2_GetComponentLocation` (`self.SpawnLocation`)) false false)))

(fn `UserConstructionScript`
  (`parent.UserConstructionScript`))