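; Base building actor for the level select map, which the player's truck drives up to for level info and interaction.
; On BeginPlay it passes level info to its interact widget and, if its quest trigger matches the current objective, becomes the truck's target and reveals its marker.
; Sphere overlap toggles the widget and sets or clears the truck's current building.
; The accessibility check is not called here, and older popup logic is left disconnected.
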(event `self.ReceiveBeginPlay`
  (bind _questtrigger (`self.QuestTrigger`))
  (bind _asbp_game_instance (cast `/Game/GameInstance/BP_GameInstance` (`GameplayStatics.GetGameInstance`)))
  (set `self.As BP Game Instance` _asbp_game_instance)
  (bind _asbp_truck_ls (cast `/Game/Blueprints/CarMovement/BP_TruckLS` (`GameplayStatics.GetPlayerPawn` 0)))
  (bind _output_get (set `self.As BP Truck LS` _asbp_truck_ls))
  (`KismetSystemLibrary.PrintString` (`|GetEnumeratorNameAsString` _questtrigger))
  (bind _asbp_eto_interect (cast `/Game/Blueprints/LevelSelect/Widgets/BP_EtoInterect` (`WidgetComponent.GetWidget` (`self.Widget`))))
  (set `/Game/Blueprints/LevelSelect/Widgets/BP_EtoInterect.LevelInformation` (`self.Level Information`) _asbp_eto_interect)
  (if (`|EnumEquality` _questtrigger (`/Game/GameInstance/BP_GameInstance.CurrentObjective` (`self.As BP Game Instance`)))
    (set `/Game/Blueprints/CarMovement/BP_TruckLS.TargetObjective` (`self.K2_GetActorLocation`) _output_get)
    (`SceneComponent.SetHiddenInGame` (`self.ObjectiveMarker`) false false)))

(event `self.Box.OnComponentBeginOverlap`
  (params (OverlappedComponent :type "PrimitiveComponent Object Reference") (OtherActor :type "Actor Object Reference") (OtherComp :type "PrimitiveComponent Object Reference") (OtherBodyIndex :type Integer) (bFromSweep :type Boolean) (SweepResult :type "HitResult Structure (by ref)"))
  ;[1 1 1] BOX COLLISION POPUP
  (set `self.Spawned` true))

(event `self.Box.OnComponentEndOverlap`
  (params (OverlappedComponent :type "PrimitiveComponent Object Reference") (OtherActor :type "Actor Object Reference") (OtherComp :type "PrimitiveComponent Object Reference") (OtherBodyIndex :type Integer))
  ;[1 1 1] BOX COLLISION POPUP
  (set `self.Spawned` false))

(event `self.Sphere.OnComponentBeginOverlap`
  (params (OverlappedComponent :type "PrimitiveComponent Object Reference") (OtherActor :type "Actor Object Reference") (OtherComp :type "PrimitiveComponent Object Reference") (OtherBodyIndex :type Integer) (bFromSweep :type Boolean) (SweepResult :type "HitResult Structure (by ref)"))
  ;[1 1 1] Updated Popup
  (bind _asbp_truck_ls (cast `/Game/Blueprints/CarMovement/BP_TruckLS` OtherActor))
  (`SceneComponent.SetVisibility` (`self.Widget`) true false)
  (set `/Game/Blueprints/CarMovement/BP_TruckLS.CurrentBuilding` self _asbp_truck_ls))

(event `self.Sphere.OnComponentEndOverlap`
  (params (OverlappedComponent :type "PrimitiveComponent Object Reference") (OtherActor :type "Actor Object Reference") (OtherComp :type "PrimitiveComponent Object Reference") (OtherBodyIndex :type Integer))
  ;[1 1 1] Updated Popup
  (bind _asbp_truck_ls (cast `/Game/Blueprints/CarMovement/BP_TruckLS` OtherActor))
  (`SceneComponent.SetVisibility` (`self.Widget`) false false)
  (set `/Game/Blueprints/CarMovement/BP_TruckLS.CurrentBuilding` null _asbp_truck_ls))

(fn `Accessible Building?`
  (returns (`IsAcessible?` :type Boolean))
  (bind _as_bp_game_instance (`self.As BP Game Instance`))
  (bind _questtrigger (`self.QuestTrigger`))
  (`/Engine/EditorBlueprintResources/StandardMacros.IsValid` (`/Game/GameInstance/BP_GameInstance.CurrentQuest` (`self.As BP Game Instance`))
    (:`Is Valid`
      (`KismetSystemLibrary.PrintString` (`|GetEnumeratorNameAsString` _questtrigger))
      (return (`|EnumEquality` (`|GetArrayItem` (`/Game/UI/Widgets/Mail/Data/PDA_Quest.Tasks` (`/Game/GameInstance/BP_GameInstance.CurrentQuest` _as_bp_game_instance)) (`/Game/GameInstance/BP_GameInstance.QuestTaskIndex` _as_bp_game_instance)) _questtrigger)))
    (:`Is Not Valid`
      (return (`|EnumEquality` (`self.BuildingType`) "NewEnumerator1")))))

(fn `UserConstructionScript`)