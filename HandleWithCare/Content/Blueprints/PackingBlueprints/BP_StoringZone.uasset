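; BP_StoringZone is the truck's drop-off zone, where the player stores packed boxes.
; Cursor hover shows an interact prompt, swaps the highlight material and enables E input, while box overlaps track packages in range.
; E stores the held package or those in range, saving each to the GameInstance with its contents' relative transforms.
; It then moves them to the mesh, disables physics, decrements PackageZone's spawn count and fires PackageStored.
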(event `self.ReceiveBeginPlay`
  (bind _asbp_third_person_character (cast `/Game/ThirdPerson/Blueprints/BP_ThirdPersonCharacter` (`GameplayStatics.GetPlayerPawn` 0)))
  (set `self.As BP Third Person Character` _asbp_third_person_character)
  (bind _asbp_game_instance (cast `/Game/GameInstance/BP_GameInstance` (`GameplayStatics.GetGameInstance`)))
  (set `self.As BP Game Instance` _asbp_game_instance)
  (bind _returnvalue (`|GenericCreateObject` "/Game/Blueprints/Widgets/WB_Interact.WB_Interact_C"))
  (set `self.InteractWidget` _returnvalue))

(event `self.Box1.OnComponentBeginOverlap`
  (params (OverlappedComponent :type "PrimitiveComponent Object Reference") (OtherActor :type "Actor Object Reference") (OtherComp :type "PrimitiveComponent Object Reference") (OtherBodyIndex :type Integer) (bFromSweep :type Boolean) (SweepResult :type "HitResult Structure (by ref)"))
  (bind _asbp_a_package (cast `/Game/Blueprints/Box/BP_A_Package` OtherActor))
  (`KismetArrayLibrary.Array_Add` (`self.PackagesInRange`) _asbp_a_package)
  (`KismetSystemLibrary.PrintString` "add")
  (`self.PackageAdded`))

(event `self.Box1.OnComponentEndOverlap`
  (params (OverlappedComponent :type "PrimitiveComponent Object Reference") (OtherActor :type "Actor Object Reference") (OtherComp :type "PrimitiveComponent Object Reference") (OtherBodyIndex :type Integer))
  (bind _asbp_a_package (cast `/Game/Blueprints/Box/BP_A_Package` OtherActor))
  (`KismetArrayLibrary.Array_RemoveItem` (`self.PackagesInRange`) _asbp_a_package)
  (`KismetSystemLibrary.PrintString` "remove"))

(event `Key|E`
  (params (Key :type "Key Structure"))
  (bind _packagesinrange (`self.PackagesInRange`))
  (bind _packagezone (`self.PackageZone`))
  (bind _array_element (`self.Array Element`))
  (bind _as_bp_third_person_character (`self.As BP Third Person Character`))
  (bind _collision (`/Game/Blueprints/ItemInteractables/BP_A_ItemInteractable.Collision` _array_element))
  (bind _output (`|GetArrayItem` (`/Game/ThirdPerson/Blueprints/BP_ThirdPersonCharacter.Items` _as_bp_third_person_character)))
  (:`Pressed`
    (`/Engine/EditorBlueprintResources/StandardMacros.IsValid` _as_bp_third_person_character
      (:`Is Valid`
        (if (`KismetSystemLibrary.DoesImplementInterface` _output "/Game/Blueprints/ItemInteractables/BlueprintInterface/BI_Package.BI_Package_C")
          (bind _asbp_a_package (cast `/Game/Blueprints/Box/BP_A_Package` (`|GetArrayItem` (`/Game/ThirdPerson/Blueprints/BP_ThirdPersonCharacter.Items` (`self.As BP Third Person Character`)))))
          (for _array_element_2 (`/Game/Blueprints/Box/BP_A_Package.InBox` _asbp_a_package)
            (`KismetArrayLibrary.Array_AddUnique` (`/Game/Blueprints/Box/BP_A_Package.ItemStruct` _asbp_a_package) (make `/Game/Blueprints/Structure/ItemStruct` (`GameplayStatics.GetObjectClass` _array_element_2) (`KismetMathLibrary.InverseTransformLocation` (`self.GetTransform` _asbp_a_package) (`self.K2_GetActorLocation` _array_element_2)) (`KismetMathLibrary.NormalizedDeltaRotator` (`self.K2_GetActorRotation` _array_element_2) (`self.K2_GetActorRotation` _asbp_a_package)))))
          (`KismetArrayLibrary.Array_AddUnique` (`/Game/GameInstance/BP_GameInstance.Packages` (`self.As BP Game Instance`)) (make `/Game/Blueprints/Structure/PackageStruct` (`GameplayStatics.GetObjectClass` _asbp_a_package) (`self.K2_GetActorLocation` _asbp_a_package) (`self.K2_GetActorRotation` _asbp_a_package) (`/Game/Blueprints/Box/BP_A_Package.ItemStruct` _asbp_a_package)))
          (`/Engine/EditorBlueprintResources/StandardMacros.DecrementInt` (`/Game/Blueprints/PackingBlueprints/BP_PackageZone.SpawnedPackages` (`self.PackageZone`))
            (:`  `
              (`self.K2_SetActorLocation` _asbp_a_package (`SceneComponent.K2_GetComponentLocation` (`self.StaticMesh`)) false false)
              (bind _collision_2 (`/Game/Blueprints/ItemInteractables/BP_A_ItemInteractable.Collision` _asbp_a_package))
              (`PrimitiveComponent.SetSimulatePhysics` _collision_2 false)
              (`PrimitiveComponent.SetCollisionResponseToChannel` _collision_2 "ECC_Visibility" "ECR_Ignore")
              (`self.PackageStored`)
              (`self.K2_DetachFromActor` _asbp_a_package "KeepWorld" "KeepWorld" "KeepWorld")
              (`KismetArrayLibrary.Array_RemoveItem` (`/Game/ThirdPerson/Blueprints/BP_ThirdPersonCharacter.Items` (`self.As BP Third Person Character`)) _asbp_a_package)))
          (elif (not (`KismetSystemLibrary.DoesImplementInterface` _output))
            (bind (_arrayindex _arrayelement) (`/Engine/EditorBlueprintResources/StandardMacros.ReverseForEachLoop` (`self.PackagesInRange`))
              (:`LoopBody`
                (for _array_element_3 (`/Game/Blueprints/Box/BP_A_Package.InBox` _arrayelement)
                  (`KismetArrayLibrary.Array_AddUnique` (`/Game/Blueprints/Box/BP_A_Package.ItemStruct` _arrayelement) (make `/Game/Blueprints/Structure/ItemStruct` (`GameplayStatics.GetObjectClass` _array_element_3) (`KismetMathLibrary.InverseTransformLocation` (`self.GetTransform` _arrayelement) (`self.K2_GetActorLocation` _array_element_3)) (`KismetMathLibrary.NormalizedDeltaRotator` (`self.K2_GetActorRotation` _array_element_3) (`self.K2_GetActorRotation` _arrayelement)))))
                (`KismetArrayLibrary.Array_AddUnique` (`/Game/GameInstance/BP_GameInstance.Packages` (`self.As BP Game Instance`)) (make `/Game/Blueprints/Structure/PackageStruct` (`GameplayStatics.GetObjectClass` _arrayelement) (`self.K2_GetActorLocation` _arrayelement) (`self.K2_GetActorRotation` _arrayelement) (`/Game/Blueprints/Box/BP_A_Package.ItemStruct` _arrayelement))))
              (:`Completed`
                (bind (_arrayindex_2 _arrayelement_2) (`/Engine/EditorBlueprintResources/StandardMacros.ReverseForEachLoop` _packagesinrange)
                  (:`LoopBody`
                    (bind (_arrayindex_3 _arrayelement_3) (`/Engine/EditorBlueprintResources/StandardMacros.ReverseForEachLoop` (`/Game/Blueprints/Box/BP_A_Package.InBox` _arrayelement_2))
                      (:`Completed`
                        (set `/Game/Blueprints/PackingBlueprints/BP_PackageZone.CanSpawnPackages?` true _packagezone)
                        (`/Engine/EditorBlueprintResources/StandardMacros.DecrementInt` (`/Game/Blueprints/PackingBlueprints/BP_PackageZone.SpawnedPackages` _packagezone)
                          (:`  `
                            (set `self.Array Element` _arrayelement_2)
                            (`KismetArrayLibrary.Array_RemoveItem` _packagesinrange _array_element)
                            (`self.K2_SetActorLocation` _array_element (`SceneComponent.K2_GetComponentLocation` (`self.StaticMesh`)) false false)
                            (`PrimitiveComponent.SetSimulatePhysics` _collision false)
                            (`PrimitiveComponent.SetCollisionResponseToChannel` _collision "ECC_Visibility" "ECR_Ignore"))))))
                  (:`Completed`
                    (`KismetSystemLibrary.PrintString` "Hello")
                    (`self.PackageStored`)))))))))))

(event `self.Box1.OnBeginCursorOver`
  (params (TouchedComponent :type "PrimitiveComponent Object Reference"))
  (bind _as_bp_third_person_character (`self.As BP Third Person Character`))
  ;[0.4554 0.2597 0.7396] Enable Interact (E) when cursor on the truck
  (`/Engine/EditorBlueprintResources/StandardMacros.IsValid` (`self.As BP Third Person Character`)
    (:`Is Valid`
      (if (not (`/Game/ThirdPerson/Blueprints/BP_ThirdPersonCharacter.IsInteracting` (`self.As BP Third Person Character`)))
        (set `/Game/ThirdPerson/Blueprints/BP_ThirdPersonCharacter.HasHoveredItem` true _as_bp_third_person_character)
        (`self.EnableInput` (`/Game/ThirdPerson/Blueprints/BP_ThirdPersonCharacter.As BP Player Controller` _as_bp_third_person_character))
        (`self.OnHover`)))))

(event `self.Box1.OnEndCursorOver`
  (params (TouchedComponent :type "PrimitiveComponent Object Reference"))
  (bind _as_bp_third_person_character (`self.As BP Third Person Character`))
  ;[0.4554 0.2597 0.7396] Disable Interact (E) when cursor off the truck
  (`/Engine/EditorBlueprintResources/StandardMacros.IsValid` (`self.As BP Third Person Character`)
    (:`Is Valid`
      (if (not (`/Game/ThirdPerson/Blueprints/BP_ThirdPersonCharacter.IsInteracting` (`self.As BP Third Person Character`)))
        (set `/Game/ThirdPerson/Blueprints/BP_ThirdPersonCharacter.HasHoveredItem` false _as_bp_third_person_character)
        (`self.DisableInput` (`/Game/ThirdPerson/Blueprints/BP_ThirdPersonCharacter.As BP Player Controller` _as_bp_third_person_character))
        (`self.OnUnhover`)))))

(fn `OnHover`
  (bind _interactwidget (`self.InteractWidget`))
  (`UserWidget.AddToViewport` _interactwidget 0)
  (set `TextBlock.Text` "[E] Store Boxes" (`/Game/Blueprints/Widgets/WB_Interact.InteractText` _interactwidget))
  (`PrimitiveComponent.SetMaterial` (`self.Plane`) 0 "/Game/Blueprints/Materials/Highlight.Highlight"))

(fn `OnUnhover`
  (`Widget.RemoveFromParent` (`self.InteractWidget`))
  (`PrimitiveComponent.SetMaterial` (`self.Plane`) 0 "/Game/Blueprints/Materials/HighlightGreen.HighlightGreen"))

(fn `UserConstructionScript`)