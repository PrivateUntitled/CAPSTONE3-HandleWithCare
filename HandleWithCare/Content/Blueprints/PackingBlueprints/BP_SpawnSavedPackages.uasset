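; Spawner that recreates the packages saved in the game instance, along with their packed items, on BeginPlay.
; Each box spawns at a random point within the Box volume, raised slightly, and drops under physics.
; Saved items spawn from stored class, location and rotation, then attach to their box with relative transforms kept.
; Items are registered in the box, owned by it, flagged packaged and draggable, and stripped of dialogue.
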(event `self.ReceiveBeginPlay`
  (bind _asbp_game_instance (cast `/Game/GameInstance/BP_GameInstance` (`GameplayStatics.GetGameInstance`)))
  (set `self.As BP Game Instance` _asbp_game_instance)
  ;[0.4549 0.2588 0.7412] Spawn New Boxes
  ;;[0.7647 0.7647 0.7647] Spawn Package
  (for _array_element (`/Game/GameInstance/BP_GameInstance.Packages` (`self.As BP Game Instance`))
    (bind ((`ClassType_29_DED2E0094CE7CE81402D5F857B8E19EF` _classtype) (`ItemStruct_27_FD7B7C76463B1372BA6C239951008261` _itemstruct)) (break `/Game/Blueprints/Structure/PackageStruct` _array_element))
    (bind _spawnedpackage (`self.Spawn Package` _classtype))
    ;;[0.7647 0.7647 0.7647] Spawn Items of Box
    (for _array_element_2 _itemstruct
      (bind _returnvalue (`|SpawnActorFromClass` (break `/Game/Blueprints/Structure/ItemStruct` _array_element_2) (`KismetMathLibrary.MakeTransform` (`.Location_6_E6A949BB445CB969F790878C051740C6` (break `/Game/Blueprints/Structure/ItemStruct` _array_element_2)) (`.Rotation_9_F1B159DE4DBA65746B89F99085B07607` (break `/Game/Blueprints/Structure/ItemStruct` _array_element_2))) "Undefined" "MultiplyWithRoot" null null))
      (`KismetArrayLibrary.Array_AddUnique` (`/Game/Blueprints/Box/BP_A_Package.InBox` _spawnedpackage) _returnvalue)
      (`self.K2_AttachToActor` _returnvalue _spawnedpackage "None" "KeepRelative" "KeepRelative" "KeepRelative" true)
      (set `/Game/Blueprints/ItemInteractables/BP_A_ItemInteractable.isPackaged` true _returnvalue)
      (set `/Game/Blueprints/ItemInteractables/BP_A_ItemInteractable.canBeDragged` true _returnvalue)
      (`self.SetOwner` _returnvalue _spawnedpackage)
      (`/Engine/EditorBlueprintResources/StandardMacros.IsValid` (`/Game/Blueprints/ItemInteractables/BP_A_ItemInteractable.Dialogue` _returnvalue)
        (:`Is Valid`
          (set `/Game/Blueprints/ItemInteractables/BP_A_ItemInteractable.Dialogue` null _returnvalue))))))

(fn `Spawn Package`
  (params (PackageToSpawn :type "/Game/Blueprints/Box/BP_A_Package Class Reference"))
  (returns (SpawnedPackage :type "/Game/Blueprints/Box/BP_A_Package Object Reference"))
  (bind _box (`self.Box`))
  (bind (_returnvalue_x _returnvalue_y _returnvalue_z) (`KismetMathLibrary.BreakVector` (`KismetMathLibrary.RandomPointInBoundingBox` (`SceneComponent.K2_GetComponentLocation` _box) (`BoxComponent.BoxExtent` _box))))
  (bind _returnvalue (`|SpawnActorFromClass` PackageToSpawn (`KismetMathLibrary.Conv_VectorToTransform` (`KismetMathLibrary.MakeVector` _returnvalue_x _returnvalue_y (+ _returnvalue_z 100.0))) "Undefined" "MultiplyWithRoot" null null))
  (bind _collision (`/Game/Blueprints/ItemInteractables/BP_A_ItemInteractable.Collision` _returnvalue))
  ;[0.7647 0.7647 0.7647] Drop Box to the Ground (Physics)
  (`PrimitiveComponent.SetCollisionEnabled` _collision "QueryAndPhysics")
  (`PrimitiveComponent.SetCollisionResponseToChannel` _collision "ECC_Visibility" "ECR_Block")
  (`PrimitiveComponent.SetSimulatePhysics` _collision true)
  (return _returnvalue))

(fn `UserConstructionScript`)