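; BP_LevelTest_Sequencer is a narrative Blueprint that resets one client's star rating when play begins.
; After the parent BeginPlay, it casts the game instance to BP_GameInstance and loops through its ClientStarData array.
; Any entry matching a hardcoded client enum value has its Stars set to zero in the stored array.
; It contains no sequencing logic of its own, and its overlap, tick and construction graphs add nothing.
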(event `self.ReceiveBeginPlay`
  (`parent.ReceiveBeginPlay`)
  (bind _asbp_game_instance (cast `/Game/GameInstance/BP_GameInstance` (`GameplayStatics.GetGameInstance`)))
  (bind _clientstardata (`/Game/GameInstance/BP_GameInstance.ClientStarData` _asbp_game_instance))
  (for (_array_element _array_index) _clientstardata
    (if (`|EnumEquality` (`.ClientName_7_4EA5C9B2469378AFECCE3DACA7E662E4` (break `/Game/GameInstance/Structures/ClientData` _array_element)) "NewEnumerator2")
      (setmembers `/Game/GameInstance/Structures/ClientData` :`StructRef` (`|GetArrayItem` _clientstardata _array_index) :`Stars` 0))))

(fn `UserConstructionScript`
  (`parent.UserConstructionScript`))