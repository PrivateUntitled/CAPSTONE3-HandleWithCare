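; Level 1 narrative sequencer that runs the packing tutorial for boxing up house items and loading them into the truck.
; On BeginPlay it sets the objective and makes the exit door ignore Visibility; if pack onboarding is unfinished, the title fade-out starts intro dialogue and a hint widget.
; Package spawned, added and stored events, gated by a step counter, plus timers advance the hints.
; The final hint's timer restores door blocking and removes the widget.
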(event `self.ReceiveBeginPlay`
  (bind _as_bp_game_instance (`self.As BP Game Instance`))
  (bind _titlecardwidget (`/Game/Blueprints/GameModes/BP_GM_Main.TitleCardWidget` (`self.As BP GM Main`)))
  (`parent.ReceiveBeginPlay`)
  (set `/Game/GameInstance/BP_GameInstance.CurrentObjective` (`self.TargetObjectiveAfter`) _as_bp_game_instance)
  (set `/Game/GameInstance/BP_GameInstance.UnpackOnboardDone` true _as_bp_game_instance)
  (bind _returnvalue (`GameplayStatics.GetActorOfClass` "/Game/Blueprints/Furniture/Doors/BP_A_ExitDoor.BP_A_ExitDoor_C"))
  (`PrimitiveComponent.SetCollisionResponseToChannel` (`/Game/Blueprints/Furniture/Doors/BP_A_ExitDoor.StaticMesh` _returnvalue) "ECC_Visibility" "ECR_Ignore")
  (`self.ShowTitle`)
  (if (not (`/Game/GameInstance/BP_GameInstance.PackOnboardDone` (`self.As BP Game Instance`)))
    (`UserWidget.BindToAnimationFinished` _titlecardwidget (`/Game/Blueprints/Widgets/WB_TitleCard.FadeOut` _titlecardwidget) (delegate `CustomEvent_0`))))

(event `CustomEvent_0`
  (`/Game/Blueprints/GameModes/BP_GM_Main.GetAllItems` (`self.As BP GM Main`))
  (`/Game/Blueprints/Narrative/AC_Narrative.AddDialogue` (`self.AC_Narrative`) "/Game/Blueprints/Narrative/DataAssets/Level1/DA_DG_Level1_Intro.DA_DG_Level1_Intro")
  (bind _returnvalue (`|CreateWidget` "/Game/Blueprints/Level1Widgets/WB_Level1Widget.WB_Level1Widget_C"))
  (bind _output_get (set `self.NewVar` _returnvalue))
  (`UserWidget.AddToViewport` _output_get 0)
  (add `/Game/Blueprints/PackingBlueprints/BP_PackageZone.PackageSpawned` (`self.NewVar_1`) (delegate `CustomEvent`)))

(event `CustomEvent_4`
  (`/Game/Blueprints/Level1Widgets/WB_Level1Widget.SetText` (`self.NewVar`) "Look around the house and place the items in the box.")
  (`KismetSystemLibrary.K2_SetTimerDelegate` (delegate `CustomEvent_1`) 15.0))

(event `CustomEvent`
  (if (== (`self.NewVar_0`) 0)
    (`/Game/Blueprints/Level1Widgets/WB_Level1Widget.SetText` (`self.NewVar`) "You can spawn in 3 boxes at a time.")
    (set `self.NewVar_0` 1)
    (`KismetSystemLibrary.K2_SetTimerDelegate` (delegate `CustomEvent_4`) 10.0)))

(event `CustomEvent_1`
  (`/Game/Blueprints/Level1Widgets/WB_Level1Widget.SetText` (`self.NewVar`) "Once done filling up the box, place it in the green zone at the entrance.")
  (add `/Game/Blueprints/PackingBlueprints/BP_StoringZone.PackageAdded` (`self.NewVar_2`) (delegate `CustomEvent_2`)))

(event `CustomEvent_2`
  (if (== (`self.NewVar_0`) 1)
    (`/Game/Blueprints/Level1Widgets/WB_Level1Widget.SetText` (`self.NewVar`) "Press E in the greenzone to store the box in the truck.")
    (set `self.NewVar_0` 2)
    (add `/Game/Blueprints/PackingBlueprints/BP_StoringZone.PackageStored` (`self.NewVar_2`) (delegate `CustomEvent_3`))))

(event `CustomEvent_3`
  (if (== (`self.NewVar_0`) 2)
    (`/Game/Blueprints/Level1Widgets/WB_Level1Widget.SetText` (`self.NewVar`) "If you need more boxes, you can always spawn more.")
    (`KismetSystemLibrary.K2_SetTimerDelegate` (delegate `CustomEvent_5`) 10.0)))

(event `CustomEvent_5`
  (`/Game/Blueprints/Level1Widgets/WB_Level1Widget.SetText` (`self.NewVar`) "When you are done, just approach the door and leave.")
  (`KismetSystemLibrary.K2_SetTimerDelegate` (delegate `CustomEvent_7`) 5.0))

(event `CustomEvent_7`
  (bind _returnvalue (`GameplayStatics.GetActorOfClass` "/Game/Blueprints/Furniture/Doors/BP_A_ExitDoor.BP_A_ExitDoor_C"))
  (`PrimitiveComponent.SetCollisionResponseToChannel` (`/Game/Blueprints/Furniture/Doors/BP_A_ExitDoor.StaticMesh` _returnvalue) "ECC_Visibility" "ECR_Block")
  (`Widget.RemoveFromParent` (`self.NewVar`)))

(fn `UserConstructionScript`
  (`parent.UserConstructionScript`))