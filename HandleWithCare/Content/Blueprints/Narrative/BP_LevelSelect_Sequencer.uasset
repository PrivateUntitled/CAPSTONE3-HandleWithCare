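; BP_LevelSelect_Sequencer runs level select narrative beats and, on BeginPlay, moves the player truck to the GameInstance's saved location if non-zero.
; The intro disables input, plays dialogue through ACNarrative, then uses a timer to blend the camera to the office building and back, followed by more dialogue and a brief tutorial widget.
; Level 1 and office events add dialogue; objective-based dispatch is disconnected, so nothing here triggers the sequences.
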(event `self.ReceiveBeginPlay`
  (bind _asbp_vehicle_truck (cast `/Game/Blueprints/CarMovement/BP_Vehicle_Truck` (`GameplayStatics.GetPlayerPawn` 0)))
  (set `self.As BP Vehicle Truck` _asbp_vehicle_truck)
  (bind _asbp_game_instance (cast `/Game/GameInstance/BP_GameInstance` (`GameplayStatics.GetGameInstance`)))
  (bind _output_get (set `self.As BP Game Instance` _asbp_game_instance))
  (bind _locationstruct (`/Game/GameInstance/BP_GameInstance.LocationStruct` _output_get))
  (if (!= (.location (break `/Game/GameInstance/Structures/LocationData` _locationstruct)) (0.0 0.0 0.0))
    (`self.K2_SetActorLocation` (`self.As BP Vehicle Truck`) (.location (break `/Game/GameInstance/Structures/LocationData` _locationstruct)) false false)))

(event `StartIntroSequence`
  (bind _ac_narrative (`self.AC_Narrative`))
  (bind _as_bp_vehicle_truck (`self.As BP Vehicle Truck`))
  (`self.DisableInput` _as_bp_vehicle_truck (`/Game/Blueprints/CarMovement/BP_Vehicle_Truck.As BP Player Controller` _as_bp_vehicle_truck))
  (`/Game/Blueprints/Narrative/AC_Narrative.AddDialogue` _ac_narrative "/Game/Blueprints/Narrative/DataAssets/LevelSelect/LevelSelect_Intro/DA_DG_LevelSelect_Intro1.DA_DG_LevelSelect_Intro1")
  (`KismetSystemLibrary.K2_SetTimerDelegate` (delegate `ShowBuilding`) (`/Game/Blueprints/Narrative/WB_Narrative.TotalTime` (`/Game/Blueprints/Narrative/AC_Narrative.Narrative` _ac_narrative))))

(event `ShowBuilding`
  (bind _as_bp_vehicle_truck (`self.As BP Vehicle Truck`))
  (bind _as_bp_player_controller (`/Game/Blueprints/CarMovement/BP_Vehicle_Truck.As BP Player Controller` _as_bp_vehicle_truck))
  (bind _returnvalue (`GameplayStatics.GetActorOfClass` "/Game/LevelSelectTest/Actors/BP_OfficeBuilding.BP_OfficeBuilding_C"))
  (`PlayerController.SetViewTargetWithBlend` _as_bp_player_controller _returnvalue 3.0 "VTBlend_Linear" 0.0 false)
  (`KismetSystemLibrary.Delay` 5.0)
  (`self.EnableInput` _as_bp_vehicle_truck _as_bp_player_controller)
  (`PlayerController.SetViewTargetWithBlend` _as_bp_player_controller _as_bp_vehicle_truck 1.0 "VTBlend_Linear" 0.0 false)
  (`KismetSystemLibrary.Delay` 1.0)
  (`/Game/Blueprints/Narrative/AC_Narrative.AddDialogue` (`self.AC_Narrative`) "/Game/Blueprints/Narrative/DataAssets/LevelSelect/LevelSelect_Intro/DA_DG_LevelSelect_Intro2.DA_DG_LevelSelect_Intro2")
  (bind _returnvalue_2 (`|GenericCreateObject` "/Game/Blueprints/Widgets/WB_TutorialWidget.WB_TutorialWidget_C"))
  (`UserWidget.AddToViewport` _returnvalue_2 0)
  (`KismetSystemLibrary.Delay` 5.0)
  (`Widget.RemoveFromParent` _returnvalue_2))

(event `StartSequenceToLevel1`
  (`/Game/Blueprints/Narrative/AC_Narrative.AddDialogue` (`self.AC_Narrative`) "/Game/Blueprints/Narrative/DataAssets/LevelSelect/LevelSelect_Level1/DA_DG_LevelSelect_Level1_Intro.DA_DG_LevelSelect_Level1_Intro"))

(event `StartSequenceToOffice`
  (`/Game/Blueprints/Narrative/AC_Narrative.AddDialogue` (`self.AC_Narrative`) "/Game/Blueprints/Narrative/DataAssets/LevelSelect/LevelSelect_Level1/DA_DG_LevelSelect_Level1_End.DA_DG_LevelSelect_Level1_End"))

(fn `UserConstructionScript`
  (`parent.UserConstructionScript`))