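; Level 2A narrative sequencer actor that runs the level's opening when play begins.
; It sets the game instance's current objective, clears its packages, and shows the title through inherited setup.
; When the title card widget's fade-out animation finishes, it calls GetAllItems on the main game mode and queues the Level 2A intro dialogue through the narrative component.
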(event `self.ReceiveBeginPlay`
  (bind _as_bp_game_instance (`self.As BP Game Instance`))
  (bind _titlecardwidget (`/Game/Blueprints/GameModes/BP_GM_Main.TitleCardWidget` (`self.As BP GM Main`)))
  (`parent.ReceiveBeginPlay`)
  (set `/Game/GameInstance/BP_GameInstance.CurrentObjective` (`self.TargetObjectiveAfter`) _as_bp_game_instance)
  (`KismetArrayLibrary.Array_Clear` (`/Game/GameInstance/BP_GameInstance.Packages` _as_bp_game_instance))
  (`self.ShowTitle`)
  (`UserWidget.BindToAnimationFinished` _titlecardwidget (`/Game/Blueprints/Widgets/WB_TitleCard.FadeOut` _titlecardwidget) (delegate `Done`)))

(event `Done`
  (`/Game/Blueprints/GameModes/BP_GM_Main.GetAllItems` (`self.As BP GM Main`))
  (`/Game/Blueprints/Narrative/AC_Narrative.AddDialogue` (`self.AC_Narrative`) "/Game/Blueprints/Narrative/DataAssets/Level2A/DA_DG_Level2A_Intro.DA_DG_Level2A_Intro"))

(fn `UserConstructionScript`
  (`parent.UserConstructionScript`))