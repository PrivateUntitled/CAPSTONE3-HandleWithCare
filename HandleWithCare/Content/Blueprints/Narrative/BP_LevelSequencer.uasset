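; BP_LevelSequencer is a narrative actor that queues dialogue as the player's level completion progresses.
; On BeginPlay it caches the game instance and main game mode, then binds CheckLevelPercentage to a percentage-check event.
; Each check compares completion against the current threshold in PercentageArray, passing the matching dialogue to ACNarrative and advancing the index, with debug prints.
; ShowTitle displays a formatted title card through the game mode.
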(event `self.ReceiveBeginPlay`
  (bind _asbp_game_instance (cast `/Game/GameInstance/BP_GameInstance` (`GameplayStatics.GetGameInstance`)))
  (set `self.As BP Game Instance` _asbp_game_instance)
  (bind _asbp_gm_main (cast `/Game/Blueprints/GameModes/BP_GM_Main` (`GameplayStatics.GetGameMode`)))
  (set `self.As BP GM Main` _asbp_gm_main)
  (add `self.CheckPercentage` (delegate `CheckLevelPercentage`)))

(event `CheckLevelPercentage`
  (bind _dialogueidx (`self.DialogueIdx`))
  (bind _returnvalue (* (`/Game/Blueprints/GameModes/BP_GM_Main.LevelCompletionPercentage` (`self.As BP GM Main`)) 100.0))
  (`KismetSystemLibrary.PrintString` (`KismetStringLibrary.Conv_DoubleToString` _returnvalue))
  (if (>= _returnvalue (`|GetArrayItem` (`self.PercentageArray`) _dialogueidx))
    (`/Game/Blueprints/Narrative/AC_Narrative.AddDialogue` (`self.AC_Narrative`) (`|GetArrayItem` (`self.Dialogues`) _dialogueidx))
    (`KismetSystemLibrary.PrintString` "WUAT")
    (set `self.DialogueIdx` (+ (`self.DialogueIdx`) 1))))

(fn `ShowTitle`
  (`/Game/Blueprints/GameModes/BP_GM_Main.ShowTitleCard` (`self.As BP GM Main`) (`|FormatText` "{Type} \n{EpName}" (`self.TitleType`) (`self.TitleName`))))

(fn `UserConstructionScript`)