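; Test car pawn driven by physics impulses and Enhanced Input.
; On BeginPlay it adds the IMC_CarControl mapping context to the possessing BP_PlayerController.
; Throttle applies a forward impulse to the mesh, then immediately zeroes its linear and angular velocity, and sets IsMoving until input completes.
; Steering yaws the mesh through local rotation, only while IsMoving is set.
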(event `self.ReceiveBeginPlay`
  (bind _asbp_player_controller (cast `/Game/Blueprints/Player/BP_PlayerController` (`self.GetController`)))
  (`EnhancedInputSubsystemInterface.AddMappingContext` (pcsubsystem `EnhancedInputLocalPlayerSubsystem` _asbp_player_controller) "/Game/Blueprints/TestingDOntMInd/IMC_CarControl.IMC_CarControl" 0 (struct)))

(event `EnhancedInput|/Game/Blueprints/TestingDOntMInd/IA_Throttle`
  (params (ActionValue :type "Float (double-precision)") (ElapsedSeconds :type "Float (double-precision)") (TriggeredSeconds :type "Float (double-precision)") (InputAction :type "InputAction Object Reference" :default "/Game/Blueprints/TestingDOntMInd/IA_Throttle.IA_Throttle"))
  (bind _staticmesh (`self.StaticMesh`))
  (bind _staticmesh_2 (`self.StaticMesh`))
  (:`Triggered`
    (set `self.isMoving` true)
    (`PrimitiveComponent.AddImpulse` _staticmesh_2 (* (`SceneComponent.GetForwardVector` _staticmesh_2) (* ActionValue (`self.ThrottleForce`))) "None" false)
    (`PrimitiveComponent.SetPhysicsLinearVelocity` _staticmesh (0.0 0.0 0.0) false "None")
    (`PrimitiveComponent.SetPhysicsAngularVelocityInRadians` _staticmesh (0.0 0.0 0.0) false "None"))
  (:`Completed`
    (set `self.isMoving` false)))

(event `EnhancedInput|/Game/Blueprints/TestingDOntMInd/IA_Steer`
  (params (ActionValue :type "Float (double-precision)") (ElapsedSeconds :type "Float (double-precision)") (TriggeredSeconds :type "Float (double-precision)") (InputAction :type "InputAction Object Reference" :default "/Game/Blueprints/TestingDOntMInd/IA_Steer.IA_Steer"))
  (:`Triggered`
    (if (`self.isMoving`)
      (`SceneComponent.K2_AddLocalRotation` (`self.StaticMesh`) (`KismetMathLibrary.MakeRotator` 0.0 0.0 (* ActionValue (`self.TurningSpeed`))) false false))))

(fn `UserConstructionScript`)