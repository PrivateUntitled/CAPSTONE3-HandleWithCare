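; Drivable truck that the player steers between buildings, with a prompt on E to confirm entering the current building's level.
; Enhanced Input throttle applies an impulse along the mesh's right vector, then zeroes linear and angular velocity; steering yaws the mesh only while throttling.
; BeginPlay creates the confirm and waypoint tracker widgets, and Tick yaws a second mesh toward TargetObjective, whose setter is unwired.
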(event Input|EnhancedActionEvents|EnhancedInputActionIA_Throttle
  (params (ActionValue :type Float%20%28double-precision%29) (ElapsedSeconds :type Float%20%28double-precision%29) (TriggeredSeconds :type Float%20%28double-precision%29) (InputAction :type Input%20Action%20Object%20Reference :default "/Game/Blueprints/CarMovement/IA_Throttle.IA_Throttle"))
  (bind _staticmesh (Variables|Default|GetStaticMesh))
  (bind _staticmesh_2 (Variables|Default|GetStaticMesh))
  (:Triggered
    (Variables|Default|SetisMoving true)
    (Physics|AddImpulse _staticmesh_2 (* (Math|Vector|GetRightVector _staticmesh_2) (* ActionValue (Variables|Default|GetThrottleForce))) "None" false)
    (Physics|SetPhysicsLinearVelocity _staticmesh "0, 0, 0" false "None")
    (Class|PrimitiveComponent|SetPhysicsAngularVelocityinRadians _staticmesh "0, 0, 0" false "None"))
  (:Completed
    (Variables|Default|SetisMoving false)))

(event Input|EnhancedActionEvents|EnhancedInputActionIA_Steer
  (params (ActionValue :type Float%20%28double-precision%29) (ElapsedSeconds :type Float%20%28double-precision%29) (TriggeredSeconds :type Float%20%28double-precision%29) (InputAction :type Input%20Action%20Object%20Reference :default "/Game/Blueprints/CarMovement/IA_Steer.IA_Steer"))
  (:Triggered
    (if (Variables|Default|GetisMoving)
      (Transformation|AddLocalRotation (Variables|Default|GetStaticMesh) (Math|Rotator|MakeRotator 0.0 0.0 (* ActionValue (Variables|Default|GetTurningSpeed))) false false))))

(event EventBeginPlay
  (bind _asbp_player_controller (Utilities|Casting|CastToBP_PlayerController (Pawn|GetController)))
  (Variables|Default|SetAs%20BP%20Player%20Controller _asbp_player_controller)
  (Input|AddMappingContext (PlayerController|LocalPlayerSubsystems|GetEnhancedInputLocalPlayerSubsystem _asbp_player_controller) "/Game/Blueprints/CarMovement/IMC_CarControl.IMC_CarControl" 0 "(bIgnoreAllPressedKeysUntilRelease=True,bForceImmediately=False)")
  (bind _returnvalue (UserInterface|CreateWidget "/Game/LevelSelectTest/Widgets/BP_LevelConfrimWidget.BP_LevelConfrimWidget_C"))
  (Variables|Default|SetConfirmWidget _returnvalue)
  (bind _returnvalue_2 (UserInterface|CreateWidget "/Game/LevelSelectTest/ObjectiveMarker/BP_WaypointMarkerDirection.BP_WaypointMarkerDirection_C"))
  (bind _output_get (Variables|Default|SetTracker _returnvalue_2))
  (UserInterface|Viewport|AddtoViewport _output_get 0))

(event EventTick
  (params (DeltaSeconds :type Float%20%28single-precision%29))
  (Transformation|SetWorldRotation (Variables|Default|GetStaticMesh1) (Math|Rotator|MakeRotator 0.0 0.0 (.yaw (Math|Rotator|FindLookatRotation (Transformation|GetWorldLocation (Variables|Default|GetStaticMesh)) (Variables|Default|GetTargetObjective)))) false false))

(event Input|KeyboardEvents|DebugKey0
  (params (Key :type Key%20Structure :default "None") (ActionValue :type Input%20Action%20Value%20Structure))
  (:Pressed
    (Default|SetMouse (Variables|Default|GetAs%20BP%20Player%20Controller) false true)))

(event Input|KeyboardEvents|E
  (params (Key :type Key%20Structure :default "None"))
  (bind _confirmwidget (Variables|Default|GetConfirmWidget))
  (bind _currentbuilding (Variables|Default|GetCurrentBuilding))
  (:Pressed
    (Utilities|IsValid _currentbuilding
      (:Is%20Valid
        (UserInterface|Viewport|AddtoViewport _confirmwidget 0)
        (Variables|/Game/LevelSelectTest/Widgets/BP_LevelConfrimWidget.BP_LevelConfrimWidget_C|SetLevelName _confirmwidget (Variables|/Game/LevelSelectTest/Actors/BP_BaseBuilding.BP_BaseBuilding_C|GetGoToLevel _currentbuilding))))))

(fn ConstructionScript)