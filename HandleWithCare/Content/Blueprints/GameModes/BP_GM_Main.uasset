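; Main game mode for a house packing and unpacking game, tracking correctly and wrongly placed items and constructing the result screen widget.
; GetAllItems starts items as wrong; CheckItemPlacements credits boxed items when packing, or sorts them by furniture category when unpacking.
; OnExitHouse saves packages and box-relative item transforms to the GameInstance for respawning or carry-over.
; OnNextLevel clears that saved list.
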(event `self.ReceiveBeginPlay`
  (bind _asbp_game_instance (cast `/Game/GameInstance/BP_GameInstance` (`GameplayStatics.GetGameInstance`)))
  (set `self.GameInstanceRef` _asbp_game_instance)
  (bind _returnvalue (`|GenericCreateObject` "/Game/Blueprints/Widgets/WB_ResultScreen.WB_ResultScreen_C"))
  (set `self.ResultScreenWidget` _returnvalue)
  (`KismetSystemLibrary.PrintString` "GMSPAWN" true true (struct :`G` 0.66 :`B` 1.0 :`A` 1.0) 5.0))

(fn `CheckItemPlacements`
  (if (`self.isPacking`)
    (bind _outactors (`GameplayStatics.GetAllActorsOfClass` "/Game/Blueprints/Box/BP_A_Package.BP_A_Package_C"))
    (for _array_element _outactors
      (for _array_element_2 (`/Game/Blueprints/Box/BP_A_Package.InBox` _array_element)
        (`/Engine/EditorBlueprintResources/StandardMacros.IsValid` _array_element_2
          (:`Is Valid`
            (`KismetArrayLibrary.Array_AddUnique` (`self.CorrectItems`) _array_element_2)
            (`KismetArrayLibrary.Array_RemoveItem` (`self.WrongItems`) _array_element_2)))))
    (else
      (bind _outactors_2 (`GameplayStatics.GetAllActorsOfClass` "/Game/Blueprints/Furniture/BP_A_Furniture.BP_A_Furniture_C"))
      (for _array_element_3 _outactors_2
        (for _array_element_4 (`/Game/Blueprints/Furniture/BP_A_Furniture.InItems` _array_element_3)
          (`/Engine/EditorBlueprintResources/StandardMacros.IsValid` _array_element_4
            (:`Is Valid`
              (if (`KismetArrayLibrary.Array_Contains` (`/Game/Blueprints/Furniture/BP_A_Furniture.AllowedItemCategories` _array_element_3) (`/Game/Blueprints/ItemInteractables/BP_A_ItemInteractable.ItemCategory` _array_element_4))
                (if (`KismetArrayLibrary.Array_Contains` (`self.WrongItems`) _array_element_4)
                  (`KismetArrayLibrary.Array_AddUnique` (`self.CorrectItems`) _array_element_4)
                  (`KismetArrayLibrary.Array_RemoveItem` (`self.WrongItems`) _array_element_4))
                (elif (`KismetArrayLibrary.Array_Contains` (`self.CorrectItems`) _array_element_4)
                  (`KismetArrayLibrary.Array_AddUnique` (`self.WrongItems`) _array_element_4)
                  (`KismetArrayLibrary.Array_RemoveItem` (`self.CorrectItems`) _array_element_4))))))))))

(fn `GetAllItems`
  (if (`self.isPacking`)
    (bind _outactors (`GameplayStatics.GetAllActorsOfClass` "/Game/Blueprints/Furniture/BP_A_Furniture.BP_A_Furniture_C"))
    (for _array_element _outactors
      (for _array_element_2 (`/Game/Blueprints/Furniture/BP_A_Furniture.InItems` _array_element)
        (`KismetArrayLibrary.Array_AddUnique` (`self.WrongItems`) _array_element_2)
        (`KismetArrayLibrary.Array_AddUnique` (`self.TotalItems`) _array_element_2)))
    (else
      (bind _outactors_2 (`GameplayStatics.GetAllActorsOfClass` "/Game/Blueprints/ItemInteractables/BP_A_ItemInteractable.BP_A_ItemInteractable_C"))
      (for _array_element_3 _outactors_2
        (if (`KismetSystemLibrary.DoesImplementInterface` _array_element_3 "/Game/Blueprints/ItemInteractables/BlueprintInterface/BI_Item_Packageable.BI_Item_Packageable_C")
          (`KismetArrayLibrary.Array_AddUnique` (`self.WrongItems`) _array_element_3)
          (`KismetArrayLibrary.Array_AddUnique` (`self.TotalItems`) _array_element_3))))))

(fn `OnExitHouse`
  (bind _outactors (`GameplayStatics.GetAllActorsOfClass` "/Game/Blueprints/Box/BP_A_Package.BP_A_Package_C"))
  (for _array_element _outactors
    (for _array_element_2 (`/Game/Blueprints/Box/BP_A_Package.InBox` _array_element)
      (`KismetArrayLibrary.Array_AddUnique` (`/Game/Blueprints/Box/BP_A_Package.ItemStruct` _array_element) (make `/Game/Blueprints/Structure/ItemStruct` (`GameplayStatics.GetObjectClass` _array_element_2) (`KismetMathLibrary.InverseTransformLocation` (`self.GetTransform` _array_element) (`self.K2_GetActorLocation` _array_element_2)) (`KismetMathLibrary.NormalizedDeltaRotator` (`self.K2_GetActorRotation` _array_element_2) (`self.K2_GetActorRotation` _array_element)))))
    (`KismetArrayLibrary.Array_AddUnique` (`/Game/GameInstance/BP_GameInstance.Packages` (`self.GameInstanceRef`)) (make `/Game/Blueprints/Structure/PackageStruct` (`GameplayStatics.GetObjectClass` _array_element) (`self.K2_GetActorLocation` _array_element) (`self.K2_GetActorRotation` _array_element) (`/Game/Blueprints/Box/BP_A_Package.ItemStruct` _array_element)))))

(fn `OnNextLevel`
  (bind _packages (`/Game/GameInstance/BP_GameInstance.Packages` (`self.GameInstanceRef`)))
  (bind (_arrayindex _arrayelement) (`/Engine/EditorBlueprintResources/StandardMacros.ReverseForEachLoop` _packages)
    (:`LoopBody`
      (`KismetArrayLibrary.Array_RemoveItem` _packages _arrayelement))))

(fn `UserConstructionScript`)