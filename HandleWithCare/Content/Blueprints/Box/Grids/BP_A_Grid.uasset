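; Grid cell actor with a Row, Column and occupied state, used for placing draggable interactable items.
; While unoccupied, its box overlap turns the grid material red when a draggable item enters and green when an item leaves.
; GetPositionXY and GetPositionYZ set its relative location on either plane from Row, Column and component bounds.
; Clicking prints its coordinates as a setup aid; Initialize, an attach helper, is marked unused.
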(event `self.ReceiveBeginPlay`
  (bind _asbp_third_person_character (cast `/Game/ThirdPerson/Blueprints/BP_ThirdPersonCharacter` (`GameplayStatics.GetPlayerPawn` 0)))
  (set `self.As BP Third Person Character` _asbp_third_person_character))

(event `self.Box.OnComponentBeginOverlap`
  (params (OverlappedComponent :type "PrimitiveComponent Object Reference") (OtherActor :type "Actor Object Reference") (OtherComp :type "PrimitiveComponent Object Reference") (OtherBodyIndex :type Integer) (bFromSweep :type Boolean) (SweepResult :type "HitResult Structure (by ref)"))
  ;[1 1 1] Change Grid color when hovered/unhovered
  (bind _asbp_a_item_interactable (cast `/Game/Blueprints/ItemInteractables/BP_A_ItemInteractable` OtherActor))
  (if (`/Game/Blueprints/ItemInteractables/BP_A_ItemInteractable.canBeDragged` _asbp_a_item_interactable)
    (if (not (`self.isOccupied`))
      (`PrimitiveComponent.SetMaterial` (`self.Grid`) 0 "/Game/Textures/GridMaterial_InstRed.GridMaterial_InstRed"))))

(event `self.Box.OnComponentEndOverlap`
  (params (OverlappedComponent :type "PrimitiveComponent Object Reference") (OtherActor :type "Actor Object Reference") (OtherComp :type "PrimitiveComponent Object Reference") (OtherBodyIndex :type Integer))
  ;[1 1 1] Change Grid color when hovered/unhovered
  (cast `/Game/Blueprints/ItemInteractables/BP_A_ItemInteractable` OtherActor)
  (if (not (`self.isOccupied`))
    (`PrimitiveComponent.SetMaterial` (`self.Grid`) 0 "/Game/Textures/GridMaterial_InstGreen.GridMaterial_InstGreen")))

(event `self.Grid.OnClicked`
  (params (TouchedComponent :type "PrimitiveComponent Object Reference") (ButtonPressed :type "Key Structure"))
  ;[1 1 1] Checks the current grid numbered when clicked (helps in setting up items)
  (`KismetSystemLibrary.PrintString` (`KismetTextLibrary.Conv_TextToString` (`|FormatText` "{Row} , {Column}" (`self.Row`) (`self.Column`)))))

(fn `GetPositionXY`
  (`self.K2_SetActorRelativeLocation` (`KismetMathLibrary.MakeVector` (* (.x (`.BoxExtent` (`KismetSystemLibrary.GetComponentBounds` (`self.BoxExtent`)))) (`self.Column`) 2.0) (* (.y (`.BoxExtent` (`KismetSystemLibrary.GetComponentBounds` (`self.BoxExtent`)))) (`self.Row`) 2.0))))

(fn `GetPositionYZ`
  (`self.K2_SetActorRelativeLocation` (`KismetMathLibrary.MakeVector` 0.0 (* (.x (`.BoxExtent` (`KismetSystemLibrary.GetComponentBounds` (`self.BoxExtent`)))) (`self.Column`) 2.0) (* (.y (`.BoxExtent` (`KismetSystemLibrary.GetComponentBounds` (`self.BoxExtent`)))) (`self.Row`) 2.0))))

(fn `Initialize`
  (params (`Scene Component` :type "SceneComponent Object Reference"))
  ;[1 0.2969 0.2969] Not being used currently
  (`/Engine/EditorBlueprintResources/StandardMacros.IsValid` (`self.GetOwner`)
    (:`Is Valid`
      (`self.K2_AttachToComponent` `Scene Component` "None" "SnapToTarget" "SnapToTarget" "KeepWorld"))))

(fn `UserConstructionScript`)