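; Clickable box actor that switches the player from roaming to a view of the box and can host a grid of cells.
; Clicking blends the view target to the box, turns off roaming on BP_PlayerController and shows the cursor.
; InitializeGrid clears old cells, then spawns a BP_A_Grid per row and column at the box's transform, passing cell size before each initializes.
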(event `self.ReceiveBeginPlay`
  (bind _asbp_third_person_character (cast `/Game/ThirdPerson/Blueprints/BP_ThirdPersonCharacter` (`GameplayStatics.GetPlayerPawn` 0)))
  (set `self.As BP Third Person Character` _asbp_third_person_character))

(event `self.Box.OnClicked`
  (params (TouchedComponent :type "PrimitiveComponent Object Reference") (ButtonPressed :type "Key Structure"))
  (bind _returnvalue (`GameplayStatics.GetPlayerController` 0))
  (`PlayerController.SetViewTargetWithBlend` _returnvalue self 0.5 "VTBlend_Linear" 0.0 false)
  (bind _asbp_player_controller (cast `/Game/Blueprints/Player/BP_PlayerController` _returnvalue))
  (set `/Game/Blueprints/Player/BP_PlayerController.Roaming` false _asbp_player_controller)
  (set `PlayerController.bShowMouseCursor` true _asbp_player_controller))

(fn `ClearGrid`
  (bind _grids (`self.Grids`))
  (if (> (`KismetArrayLibrary.Array_Length` (`self.Grids`)) 0)
    (bind (_arrayindex _arrayelement) (`/Engine/EditorBlueprintResources/StandardMacros.ReverseForEachLoop` _grids)
      (:`LoopBody`
        (`self.K2_DestroyActor` _arrayelement))
      (:`Completed`
        (`KismetArrayLibrary.Array_Clear` _grids)))))

(fn `InitializeGrid`
  (`self.ClearGrid`)
  (for _index (range (`self.Rows`))
    (for _index_2 (range (`self.Columns`))
      (bind _returnvalue (`|SpawnActorFromClass` "/Game/Blueprints/Box/BP_A_Grid.BP_A_Grid_C" (`KismetMathLibrary.MakeTransform` (`self.K2_GetActorLocation`) (`self.K2_GetActorRotation`)) "AlwaysSpawn" "MultiplyWithRoot" self _index _index_2 null))
      (set `/Game/Blueprints/Box/BP_A_Grid.GridCellSize` (`self.GridCellSize`) _returnvalue)
      (`/Game/Blueprints/Box/BP_A_Grid.Initialize` _returnvalue null)
      (`KismetArrayLibrary.Array_Add` (`self.Grids`) _returnvalue))))

(fn `UserConstructionScript`)