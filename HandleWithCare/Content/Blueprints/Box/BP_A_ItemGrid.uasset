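; Single grid cell actor, apparently for placing items in the player's box.
; Initialize, when an owner exists, attaches the cell to a supplied scene component, scales its Grid component by GridCellSize and offsets it by Row and Column using the component's bounds.
; BeginPlay caches the third-person character and the original grid material.
; Cursor and overlap events are empty; logic setting the current box's CurrentGrid is disconnected.
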(event `self.ReceiveBeginPlay`
  (bind _asbp_third_person_character (cast `/Game/ThirdPerson/Blueprints/BP_ThirdPersonCharacter` (`GameplayStatics.GetPlayerPawn` 0)))
  (set `self.As BP Third Person Character` _asbp_third_person_character)
  (set `self.Original Material` "/Game/Textures/GridMaterial.GridMaterial"))

(event `self.Grid.OnBeginCursorOver`
  (params (TouchedComponent :type "PrimitiveComponent Object Reference")))

(event `self.Grid.OnEndCursorOver`
  (params (TouchedComponent :type "PrimitiveComponent Object Reference")))

(event `self.Box.OnComponentBeginOverlap`
  (params (OverlappedComponent :type "PrimitiveComponent Object Reference") (OtherActor :type "Actor Object Reference") (OtherComp :type "PrimitiveComponent Object Reference") (OtherBodyIndex :type Integer) (bFromSweep :type Boolean) (SweepResult :type "HitResult Structure (by ref)")))

(fn `Initialize`
  (params (`Scene Component` :type "SceneComponent Object Reference"))
  (bind _gridcellsize (`self.GridCellSize`))
  (`/Engine/EditorBlueprintResources/StandardMacros.IsValid` (`self.GetOwner`)
    (:`Is Valid`
      (`self.K2_AttachToComponent` `Scene Component` "None" "SnapToTarget" "SnapToTarget" "KeepRelative")
      (`SceneComponent.SetRelativeScale3D` (`self.Grid`) (`KismetMathLibrary.MakeVector` _gridcellsize _gridcellsize 1.0))
      (`self.K2_SetActorRelativeLocation` (`KismetMathLibrary.MakeVector` (* (.x (`.BoxExtent` (`KismetSystemLibrary.GetComponentBounds` (`self.Grid`)))) (`self.Column`) 2.0) (* (.y (`.BoxExtent` (`KismetSystemLibrary.GetComponentBounds` (`self.Grid`)))) (`self.Row`) 2.0))))))

(fn `UserConstructionScript`)