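; Package box actor that the player can click to pick up, or open with E while hovering if it is not already carried.
; Opening switches the view to the box, hides the character, shows WB_BoxUI and lays out carried items, chaining each from the previous item's Arrow.
; GetOutBoxItems returns OutBox items to the character's platform.
; InitializeGrid rebuilds a row-by-column grid of BP_A_Grid cells.
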(event `self.ReceiveBeginPlay`
  (`parent.ReceiveBeginPlay`)
  (bind _returnvalue (`|GenericCreateObject` "/Game/Blueprints/Player/PlayerUI/WB_BoxUI.WB_BoxUI_C"))
  (set `self.BoxWidget` _returnvalue))

(event `self.ReceiveActorBeginOverlap`
  (params (OtherActor :type "Actor Object Reference"))
  (`parent.ReceiveActorBeginOverlap` null))

(event `self.Collision.OnBeginCursorOver`
  (params (TouchedComponent :type "PrimitiveComponent Object Reference"))
  (`self.On Hover`)
  (`self.EnableInput` (`/Game/ThirdPerson/Blueprints/BP_ThirdPersonCharacter.As BP Player Controller` (`self.As BP Third Person Character`))))

(event `self.Collision.OnEndCursorOver`
  (params (TouchedComponent :type "PrimitiveComponent Object Reference"))
  (`self.OnUnhover`)
  (`self.DisableInput` (`/Game/ThirdPerson/Blueprints/BP_ThirdPersonCharacter.As BP Player Controller` (`self.As BP Third Person Character`))))

(event `self.Collision.OnClicked`
  (params (TouchedComponent :type "PrimitiveComponent Object Reference") (ButtonPressed :type "Key Structure"))
  (`/Game/Blueprints/Player/BP_AC_PickUp.PickupItem` (`/Game/ThirdPerson/Blueprints/BP_ThirdPersonCharacter.BP_AC_PickUp` (`self.As BP Third Person Character`))))

(event `ShowOptions`
  (bind _returnvalue (`|GenericCreateObject` "/Game/Blueprints/Player/PlayerUI/WB_BoxOptions.WB_BoxOptions_C"))
  (`UserWidget.AddToViewport` _returnvalue 0))

(event `OpenBox`
  (bind _as_bp_third_person_character (`self.As BP Third Person Character`))
  (bind _collision (`self.Collision`))
  (bind _items (`/Game/ThirdPerson/Blueprints/BP_ThirdPersonCharacter.Items` (`self.As BP Third Person Character`)))
  (`PlayerController.SetViewTargetWithBlend` (`/Game/ThirdPerson/Blueprints/BP_ThirdPersonCharacter.As BP Player Controller` _as_bp_third_person_character) self 0.0 "VTBlend_Linear" 0.0 false)
  (`PrimitiveComponent.SetSimulatePhysics` _collision false)
  (`PrimitiveComponent.SetCollisionEnabled` _collision "NoCollision")
  (`UserWidget.AddToViewport` (`self.BoxWidget`) 0)
  (`self.SetActorHiddenInGame` _as_bp_third_person_character true)
  (`self.GetItems` (`self.ItemSpawnLocation`) _items)
  (set `self.OutBox` _items)
  (set `/Game/ThirdPerson/Blueprints/BP_ThirdPersonCharacter.InteractingBox` true (`self.As BP Third Person Character`))
  (`PrimitiveComponent.SetCollisionEnabled` (`self.Box`) "QueryOnly")
  (set `self.isInteracted` true)
  (for _array_element (`self.InBox`)
    (`PrimitiveComponent.SetCollisionEnabled` (`/Game/Blueprints/ItemInteractables/BP_A_ItemInteractable.Collision` _array_element) "QueryOnly")))

(event `Key|E`
  (params (Key :type "Key Structure"))
  (bind _as_bp_third_person_character (`self.As BP Third Person Character`))
  (:`Pressed`
    (if (not (`KismetArrayLibrary.Array_Contains` (`/Game/ThirdPerson/Blueprints/BP_ThirdPersonCharacter.Items` (`self.As BP Third Person Character`)) self))
      (`self.OpenBox`)
      (`/Game/Blueprints/Player/BP_PlayerController.SetMouse` (`/Game/ThirdPerson/Blueprints/BP_ThirdPersonCharacter.As BP Player Controller` _as_bp_third_person_character) false true)
      (set `/Game/ThirdPerson/Blueprints/BP_ThirdPersonCharacter.CurrentBox` self _as_bp_third_person_character)
      (`KismetSystemLibrary.PrintString` "EEEEE")
      (`self.EnableInput` (`/Game/ThirdPerson/Blueprints/BP_ThirdPersonCharacter.As BP Player Controller` (`self.As BP Third Person Character`))))))

(event `GetItems`
  (params (`Static Mesh Component` :type "StaticMeshComponent Object Reference") (Items :type "Array of /Game/Blueprints/ItemInteractables/BP_A_ItemInteractable Object Reference"))
  (for (_array_element _array_index) Items
    (if (== _array_index 0)
      (`self.K2_DetachFromActor` _array_element "KeepWorld" "KeepWorld" "KeepWorld")
      (`self.K2_SetActorLocation` _array_element (`SceneComponent.K2_GetComponentLocation` `Static Mesh Component`) false false)
      (`self.K2_SetActorRotation` _array_element (`self.K2_GetActorRotation`) false)
      (else
        (bind _output (`|GetArrayItem` Items _array_index))
        (`self.K2_DetachFromActor` _output "KeepWorld" "KeepWorld" "KeepWorld")
        (`self.K2_SetActorLocation` _output (`SceneComponent.K2_GetComponentLocation` (`/Game/Blueprints/ItemInteractables/BP_A_ItemInteractable.Arrow` (`|GetArrayItem` Items (- _array_index 1)))) false false)
        (`self.K2_SetActorRotation` :`self` _output)))))

(event `GetOutBoxItems`
  (bind _outbox (`self.OutBox`))
  (bind _sm_assetplatform (`/Game/ThirdPerson/Blueprints/BP_ThirdPersonCharacter.SM_AssetPlatform` (`self.As BP Third Person Character`)))
  (`self.GetItems` _sm_assetplatform _outbox)
  (for _array_element _outbox
    (`self.K2_AttachToComponent` _array_element _sm_assetplatform "None" "KeepWorld" "KeepWorld" "KeepWorld" true)))

(fn `ClearGrid`
  (bind _grids_0 (`self.Grids_0`))
  (if (> (`KismetArrayLibrary.Array_Length` (`self.Grids_0`)) 0)
    (bind (_arrayindex _arrayelement) (`/Engine/EditorBlueprintResources/StandardMacros.ReverseForEachLoop` _grids_0)
      (:`LoopBody`
        (`self.K2_DestroyActor` _arrayelement))
      (:`Completed`
        (`KismetArrayLibrary.Array_Clear` _grids_0)))))

(fn `InitializeGrid`
  (`self.ClearGrid`)
  (for _index (range (`self.Rows_0`))
    (for _index_2 (range (`self.Columns_0`))
      (bind _returnvalue (`|SpawnActorFromClass` "/Game/Blueprints/Box/BP_A_Grid.BP_A_Grid_C" (`KismetMathLibrary.MakeTransform` (`self.K2_GetActorLocation`) (`self.K2_GetActorRotation`)) "AlwaysSpawn" "MultiplyWithRoot" self _index _index_2 null))
      (set `/Game/Blueprints/Box/BP_A_Grid.GridCellSize` (`self.GridCellSize_0`) _returnvalue)
      (`/Game/Blueprints/Box/BP_A_Grid.Initialize` _returnvalue (`self.GridAdjustor`))
      (`KismetArrayLibrary.Array_Add` (`self.Grids_0`) _returnvalue))))

(fn `UserConstructionScript`
  (`parent.UserConstructionScript`))