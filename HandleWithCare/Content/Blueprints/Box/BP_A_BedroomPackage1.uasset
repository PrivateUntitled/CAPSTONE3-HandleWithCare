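; A bedroom moving-box variant that starts pre-packed with books of several sizes and shirts.
; On BeginPlay, after the parent setup, it calls BPACPopulateItems repeatedly to place each item type in its own region of the box's first grid, rotating some books.
; It then flags every item in InBox as packaged.
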(event `self.ReceiveBeginPlay`
  (`parent.ReceiveBeginPlay`)
  (`/Game/Blueprints/Player/BP_AC_PopulateItems.PopulateItems` (`self.BP_AC_PopulateItems`) (`self.Grids_0`) 0 0 1 0 (struct :`Yaw` -90.0) "/Game/Blueprints/ItemInteractables/BP_A_BookChonk.BP_A_BookChonk_C" 3 self (`self.InBox`))
  (`/Game/Blueprints/Player/BP_AC_PopulateItems.PopulateItems` :`self` (`self.BP_AC_PopulateItems`) :`Grid` (`self.Grids_0`) :`InitialRow` 4 :`EndRow` 5 :`EndColumn` 2 :`Item` "/Game/Blueprints/ItemInteractables/BP_A_Shirt.BP_A_Shirt_C" :`NumberOfItems` 2 :`ActorAttached` self :`InItems` (`self.InBox`))
  (`/Game/Blueprints/Player/BP_AC_PopulateItems.PopulateItems` :`self` (`self.BP_AC_PopulateItems`) :`Grid` (`self.Grids_0`) :`InitialRow` 3 :`EndRow` 3 :`EndColumn` 1 :`Item` "/Game/Blueprints/ItemInteractables/BP_A_BookTall.BP_A_BookTall_C" :`NumberOfItems` 5 :`ActorAttached` self :`InItems` (`self.InBox`))
  (`/Game/Blueprints/Player/BP_AC_PopulateItems.PopulateItems` (`self.BP_AC_PopulateItems`) (`self.Grids_0`) 1 2 2 2 (struct :`Yaw` -90.0) "/Game/Blueprints/ItemInteractables/BP_A_BookSmall.BP_A_BookSmall_C" 5 self (`self.InBox`))
  (`/Game/Blueprints/Player/BP_AC_PopulateItems.PopulateItems` :`self` (`self.BP_AC_PopulateItems`) :`Grid` (`self.Grids_0`) :`InitialColumn` 1 :`EndColumn` 2 :`Item` "/Game/Blueprints/ItemInteractables/BP_A_BookNormal.BP_A_BookNormal_C" :`NumberOfItems` 5 :`ActorAttached` self :`InItems` (`self.InBox`))
  (for _array_element (`self.InBox`)
    (set `/Game/Blueprints/ItemInteractables/BP_A_ItemInteractable.isPackaged` true _array_element)))

(fn `UserConstructionScript`
  (`parent.UserConstructionScript`))