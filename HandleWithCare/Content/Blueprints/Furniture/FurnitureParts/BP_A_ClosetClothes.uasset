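; Clothes part of a BP_A_Closet that dispenses a shirt when its mesh is clicked.
; A click spawns a BP_A_Shirt at the owning closet's item location, records it in OutItems, and switches the slot to an empty, red-highlighted state.
; SwitchMesh sets material and Visibility collision, so empty slots ignore clicks; switching back to filled also removes and destroys the given item.
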(event `self.ReceiveBeginPlay`
  (`KismetSystemLibrary.PrintString` (`KismetSystemLibrary.GetDisplayName` (`self.GetOwner`))))

(event `self.ClothesCollisionBox.OnComponentHit`
  (params (HitComponent :type "PrimitiveComponent Object Reference") (OtherActor :type "Actor Object Reference") (OtherComp :type "PrimitiveComponent Object Reference") (NormalImpulse :type "Vector Structure") (Hit :type "HitResult Structure (by ref)")))

(event `self.ClothesCollisionBox.OnClicked`
  (params (TouchedComponent :type "PrimitiveComponent Object Reference") (ButtonPressed :type "Key Structure")))

(event `self.StaticMesh.OnClicked`
  (params (TouchedComponent :type "PrimitiveComponent Object Reference") (ButtonPressed :type "Key Structure"))
  (if (`self.hasMesh`)
    (bind _asbp_a_closet (cast `/Game/Blueprints/Furniture/BP_A_Closet` (`self.GetOwner`)))
    (bind _returnvalue (`|SpawnActorFromClass` "/Game/Blueprints/ItemInteractables/BP_A_Shirt.BP_A_Shirt_C" (`KismetMathLibrary.MakeTransform` (`SceneComponent.K2_GetComponentLocation` (`/Game/Blueprints/Furniture/BP_A_Furniture.ItemInitialLocation` _asbp_a_closet)) (`self.K2_GetActorRotation` _asbp_a_closet)) "Undefined" "MultiplyWithRoot" null null))
    (`KismetArrayLibrary.Array_Add` (`/Game/Blueprints/Furniture/BP_A_Furniture.OutItems` _asbp_a_closet) _returnvalue)
    (`self.SwitchMesh` false null "/Game/Blueprints/Materials/HighlightRed.HighlightRed")))

(fn `SwitchMesh`
  (params (hasMesh :type Boolean) (Target :type "/Game/Blueprints/ItemInteractables/BP_A_ItemInteractable Object Reference") (Material :type "MaterialInterface Object Reference"))
  (`PrimitiveComponent.SetMaterial` (`self.StaticMesh`) 0 Material)
  (bind _output_get (set `self.hasMesh` hasMesh))
  (if _output_get
    (`PrimitiveComponent.SetCollisionResponseToChannel` (`self.StaticMesh`) "ECC_Visibility" "ECR_Block")
    (bind _asbp_a_closet (cast `/Game/Blueprints/Furniture/BP_A_Closet` (`self.GetOwner`)))
    (`KismetArrayLibrary.Array_RemoveItem` (`/Game/Blueprints/Furniture/BP_A_Furniture.OutItems` _asbp_a_closet) Target)
    (`self.K2_DestroyActor` Target)
    (else
      (`PrimitiveComponent.SetCollisionResponseToChannel` (`self.StaticMesh`) "ECC_Visibility" "ECR_Ignore"))))

(fn `UserConstructionScript`)