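; BP_A_SwitchableItems is a furniture part that acts as a slot for one item, showing occupancy through its mesh material.
; SwitchMesh sets material and Visibility collision; when filling, it registers the target in the owning closet's InItems and moves it to a fixed below-origin location.
; Clicking a filled slot returns the item to the owning furniture's initial location, moves it to OutItems and highlights the slot red.
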(event `self.ReceiveBeginPlay`)

(event `self.StaticMesh.OnClicked`
  (params (TouchedComponent :type "PrimitiveComponent Object Reference") (ButtonPressed :type "Key Structure"))
  (bind _currentitem (`self.CurrentItem`))
  (if (`self.hasMesh`)
    (bind _asbp_a_furniture (cast `/Game/Blueprints/Furniture/BP_A_Furniture` (`self.GetOwner`)))
    (`self.K2_SetActorLocationAndRotation` _currentitem (`SceneComponent.K2_GetComponentLocation` (`/Game/Blueprints/Furniture/BP_A_Furniture.ItemInitialLocation` _asbp_a_furniture)) (`self.K2_GetActorRotation` _asbp_a_furniture) false false)
    (`KismetArrayLibrary.Array_AddUnique` (`/Game/Blueprints/Furniture/BP_A_Furniture.OutItems` _asbp_a_furniture) _currentitem)
    (`KismetArrayLibrary.Array_RemoveItem` (`/Game/Blueprints/Furniture/BP_A_Furniture.InItems` _asbp_a_furniture) (`self.CurrentItem`))
    (set `self.CurrentItem` null)
    (`self.SwitchMesh` false null "/Game/Blueprints/Materials/HighlightRed.HighlightRed")))

(fn `SwitchMesh`
  (params (hasMesh :type Boolean) (Target :type "/Game/Blueprints/ItemInteractables/BP_A_ItemInteractable Object Reference") (Material :type "MaterialInterface Object Reference"))
  (`PrimitiveComponent.SetMaterial` (`self.StaticMesh`) 0 Material)
  (bind _output_get (set `self.hasMesh` hasMesh))
  (if _output_get
    (`PrimitiveComponent.SetCollisionResponseToChannel` (`self.StaticMesh`) "ECC_Visibility" "ECR_Block")
    (bind _asbp_a_closet (cast `/Game/Blueprints/Furniture/BP_A_Closet` (`self.GetOwner`)))
    (`/Engine/EditorBlueprintResources/StandardMacros.IsValid` Target
      (:`Is Valid`
        (`KismetArrayLibrary.Array_RemoveItem` (`/Game/Blueprints/Furniture/BP_A_Furniture.OutItems` _asbp_a_closet) Target)
        (`KismetArrayLibrary.Array_AddUnique` (`/Game/Blueprints/Furniture/BP_A_Furniture.InItems` _asbp_a_closet) Target)
        (bind _output_get_2 (set `self.CurrentItem` Target))
        (`self.K2_SetActorLocation` _output_get_2 (0.0 0.0 -50.0) false false)))
    (else
      (`PrimitiveComponent.SetCollisionResponseToChannel` (`self.StaticMesh`) "ECC_Visibility" "ECR_Ignore"))))

(fn `UserConstructionScript`)