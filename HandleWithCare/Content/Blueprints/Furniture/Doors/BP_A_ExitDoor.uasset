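; Exit door actor that lets the player leave the level.
; Hovering the cursor over its mesh highlights it, shows an "E To Exit" prompt and enables its input.
; Pressing E shows the game mode's result screen if level completion is full.
; Otherwise it opens the exit door widget and disables the player character's input.
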(event `self.ReceiveBeginPlay`
  (bind _returnvalue (`|GenericCreateObject` "/Game/Blueprints/Widgets/WB_Interact.WB_Interact_C"))
  (set `self.InteractWidget` _returnvalue)
  (bind _returnvalue_2 (`|GenericCreateObject` "/Game/Blueprints/Widgets/WB_ExitDoor.WB_ExitDoor_C"))
  (set `self.ExitDoorWidget` _returnvalue_2)
  (bind _asbp_third_person_character (cast `/Game/ThirdPerson/Blueprints/BP_ThirdPersonCharacter` (`GameplayStatics.GetPlayerPawn` 0)))
  (set `self.As BP Third Person Character` _asbp_third_person_character)
  (bind _asbp_gm_main (cast `/Game/Blueprints/GameModes/BP_GM_Main` (`GameplayStatics.GetGameMode`)))
  (set `self.As BP GM Main` _asbp_gm_main))

(event `self.StaticMesh.OnBeginCursorOver`
  (params (TouchedComponent :type "PrimitiveComponent Object Reference"))
  (if (not (`Widget.IsInViewport` (`self.ExitDoorWidget`)))
    (`self.OnHover`)
    (`self.EnableInput` (`/Game/ThirdPerson/Blueprints/BP_ThirdPersonCharacter.As BP Player Controller` (`self.As BP Third Person Character`)))))

(event `self.StaticMesh.OnEndCursorOver`
  (params (TouchedComponent :type "PrimitiveComponent Object Reference"))
  (`self.OnUnhover`)
  (`self.DisableInput` (`/Game/ThirdPerson/Blueprints/BP_ThirdPersonCharacter.As BP Player Controller` (`self.As BP Third Person Character`))))

(event `Key|E`
  (params (Key :type "Key Structure"))
  (bind _as_bp_third_person_character (`self.As BP Third Person Character`))
  (:`Pressed`
    (if (!= (`/Game/Blueprints/GameModes/BP_GM_Main.LevelCompletionPercentage` (`self.As BP GM Main`)) 1.0)
      (`UserWidget.AddToViewport` (`self.ExitDoorWidget`) 0)
      (`self.DisableInput` _as_bp_third_person_character (`/Game/ThirdPerson/Blueprints/BP_ThirdPersonCharacter.As BP Player Controller` _as_bp_third_person_character))
      (else
        (`UserWidget.AddToViewport` (`/Game/Blueprints/GameModes/BP_GM_Main.ResultScreenWidget` (`self.As BP GM Main`)) 0)))))

(fn `OnHover`
  (bind _interactwidget (`self.InteractWidget`))
  (`UserWidget.AddToViewport` _interactwidget 0)
  (set `TextBlock.Text` "E To Exit" (`/Game/Blueprints/Widgets/WB_Interact.InteractText` _interactwidget))
  (`PrimitiveComponent.SetMaterial` (`self.StaticMesh`) 0 "/Game/Blueprints/Materials/Highlight.Highlight"))

(fn `OnUnhover`
  (`Widget.RemoveFromParent` (`self.InteractWidget`))
  (`PrimitiveComponent.SetMaterial` (`self.StaticMesh`) 0 null))

(fn `UserConstructionScript`)