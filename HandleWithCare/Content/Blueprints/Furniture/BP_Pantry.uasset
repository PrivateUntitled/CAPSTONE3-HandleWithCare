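; BP_Pantry is a furniture Blueprint for a pantry with a swinging door and seven grid areas.
; The construction script builds a small grid on each area's scene component through InitializeGrid, and BeginPlay collects those grids into GridStruct.
; The open and close events extend the parent's logic, each playing its own timeline that lerps the door's yaw between closed and open angles.
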(event `self.ReceiveBeginPlay`
  (bind _gridstruct (`self.GridStruct`))
  (`parent.ReceiveBeginPlay`)
  (`KismetArrayLibrary.Array_Add` _gridstruct (make `/Game/Blueprints/Structure/GridStruct` (`self.Grids1`)))
  (`KismetArrayLibrary.Array_Add` _gridstruct (make `/Game/Blueprints/Structure/GridStruct` (`self.Grids2`)))
  (`KismetArrayLibrary.Array_Add` _gridstruct (make `/Game/Blueprints/Structure/GridStruct` (`self.Grids3`)))
  (`KismetArrayLibrary.Array_Add` _gridstruct (make `/Game/Blueprints/Structure/GridStruct` (`self.Grids4`)))
  (`KismetArrayLibrary.Array_Add` _gridstruct (make `/Game/Blueprints/Structure/GridStruct` (`self.Grids5`)))
  (`KismetArrayLibrary.Array_Add` _gridstruct (make `/Game/Blueprints/Structure/GridStruct` (`self.Grids6`)))
  (`KismetArrayLibrary.Array_Add` _gridstruct (make `/Game/Blueprints/Structure/GridStruct` (`self.Grids7`))))

(event `self.OpenFurniture`
  (`parent.OpenFurniture`)
  (bind (_direction _leftdooropen) (`Timeline|Timeline` :!via `PlayFromStart` :!label _label)
    (:`Update`
      (`SceneComponent.K2_SetRelativeRotation` (`self.Door`) (`KismetMathLibrary.MakeRotator` 0.0 0.0 (`KismetMathLibrary.Lerp` (`self.DoorCloseFloat`) (`self.DoorOpenFloat`) _leftdooropen)) false false)
      (bind (_direction_2 _leftdooropen_2) (`Timeline|Timeline_1` :!via `Stop` :!label _label_2)
        (:`Update`
          (`SceneComponent.K2_SetRelativeRotation` (`self.Door`) (`KismetMathLibrary.MakeRotator` 0.0 0.0 (`KismetMathLibrary.Lerp` (`self.DoorOpenFloat`) (`self.DoorCloseFloat`) _leftdooropen_2)) false false)
          (goto _label :!via `Stop`))))))

(event `self.OnFurnitureClose`
  (`parent.OnFurnitureClose`)
  (goto _label_2 :!via `PlayFromStart`))

(fn `UserConstructionScript`
  (`parent.UserConstructionScript`)
  (`self.InitializeGrid` 2 2 (`self.Grid1`) (`self.Grids1`))
  (`self.InitializeGrid` 2 2 (`self.Grid2`) (`self.Grids2`))
  (`self.InitializeGrid` 2 2 (`self.Grid3`) (`self.Grids3`))
  (`self.InitializeGrid` 2 2 (`self.Grid4`) (`self.Grids4`))
  (`self.InitializeGrid` 2 2 (`self.Grid5`) (`self.Grids5`))
  (`self.InitializeGrid` 2 2 (`self.Grid6`) (`self.Grids6`))
  (`self.InitializeGrid` 2 2 (`self.Grid7`) (`self.Grids7`)))