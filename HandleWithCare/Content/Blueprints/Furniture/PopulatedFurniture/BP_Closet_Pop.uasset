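; BP_Closet_Pop is a populated closet furniture Blueprint that sets up the clothes it holds when play begins.
; After the parent BeginPlay, it loops over the Shirts array, casts each element to BP_A_ClosetClothes and calls SwitchMesh with a mesh enabled and the M_Basic_Wall material.
; The construction script only calls its parent, and the overlap and tick events are disabled.
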(event `self.ReceiveBeginPlay`
  (`parent.ReceiveBeginPlay`)
  (for _array_element (`self.Shirts`)
    (bind _asbp_a_closet_clothes (cast `/Game/Blueprints/Furniture/FurnitureParts/BP_A_ClosetClothes` _array_element))
    (`/Game/Blueprints/Furniture/FurnitureParts/BP_A_ClosetClothes.SwitchMesh` _asbp_a_closet_clothes true null "/Game/StarterContent/Materials/M_Basic_Wall.M_Basic_Wall")))

(fn `UserConstructionScript`
  (`parent.UserConstructionScript`))