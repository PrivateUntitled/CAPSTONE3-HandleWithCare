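; Pre-populated table furniture variant that fills itself with books and plates when play begins.
; After the parent BeginPlay, it calls PopulateItems on BPACPopulateItems twice, once per item class, each targeting its own cell range of the same Grids1 grid.
; The table passes itself as the actor the items attach to, and its construction script only calls the parent.
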(event `self.ReceiveBeginPlay`
  (`parent.ReceiveBeginPlay`)
  (`/Game/Blueprints/Player/BP_AC_PopulateItems.PopulateItems` :`self` (`self.BP_AC_PopulateItems`) :`Grid` (`self.Grids1`) :`InitialColumn` 1 :`EndColumn` 3 :`Item` "/Game/Blueprints/ItemInteractables/BP_A_BookNormal.BP_A_BookNormal_C" :`NumberOfItems` 2 :`ActorAttached` self :`InItems` (`self.InItems`))
  (`/Game/Blueprints/Player/BP_AC_PopulateItems.PopulateItems` :`self` (`self.BP_AC_PopulateItems`) :`Grid` (`self.Grids1`) :`InitialRow` 5 :`EndColumn` 2 :`EndRow` 7 :`Item` "/Game/Blueprints/ItemInteractables/BP_A_Plate.BP_A_Plate_C" :`NumberOfItems` 5 :`ActorAttached` self :`InItems` (`self.InItems`)))

(fn `UserConstructionScript`
  (`parent.UserConstructionScript`))