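; Populated variant of a cabinet drawer furniture Blueprint that fills its inventory grids with preset items when play begins.
; After the parent BeginPlay, it loops through ItemsToPopulate, matching each entry by index to a grid in GridStruct.
; Each placement's cell range, rotation, item and count go to BPACPopulateItems with the drawer as attached actor.
; Row and column values are swapped in that call.
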(event `self.ReceiveBeginPlay`
  (`parent.ReceiveBeginPlay`)
  (for (_array_element _array_index) (`self.ItemsToPopulate`)
    (for _array_element_2 (`/Game/Blueprints/DataAssets/PopulateItemsDataAssets/DA_PopulateItems.PopulateItemsStruct` _array_element)
      (bind _output_grid (break `/Game/Blueprints/Structure/GridStruct` (`|GetArrayItem` (`self.GridStruct`) _array_index)))
      (`/Game/Blueprints/Player/BP_AC_PopulateItems.PopulateItems` (`self.BP_AC_PopulateItems`) _output_grid (`.InitialColumn_12_08EABF644FC0E26138F02B9625A10D3A` (break `/Game/Blueprints/Structure/PopulateItemsStruct` _array_element_2)) (break `/Game/Blueprints/Structure/PopulateItemsStruct` _array_element_2) (`.EndColumn_16_2CEB51A9439026185000C7BC82E190C3` (break `/Game/Blueprints/Structure/PopulateItemsStruct` _array_element_2)) (`.EndRow_14_7A8B15EE445E8A2B1BB91BA963DD0099` (break `/Game/Blueprints/Structure/PopulateItemsStruct` _array_element_2)) (`.Rotation_19_CBE0018B421A55AA5758EEA9B1EBAAAD` (break `/Game/Blueprints/Structure/PopulateItemsStruct` _array_element_2)) (`.Item_22_A1880C41486790E2DAEA9D81E4BCEC38` (break `/Game/Blueprints/Structure/PopulateItemsStruct` _array_element_2)) (`.NumberOfItems_25_21A11A934D797545D7F408A99A6CAEC9` (break `/Game/Blueprints/Structure/PopulateItemsStruct` _array_element_2)) self (`self.InItems`)))))

(fn `UserConstructionScript`
  (`parent.UserConstructionScript`))