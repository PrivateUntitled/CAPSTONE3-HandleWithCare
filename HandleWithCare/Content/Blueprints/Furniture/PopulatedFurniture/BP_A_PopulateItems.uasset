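; Level setup actor that fills the world with starting items for either a packing or a non-packing game, based on its IsPacking flag.
; On BeginPlay it copies that flag to BP_GM_Main, then has every furniture actor (packing) or every package (otherwise) populate its items.
; It then flags the contained items as in furniture or packaged and calls GetAllItems on the game mode.
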(event `self.ReceiveBeginPlay`
  (bind _furnitures (`self.Furnitures`))
  (bind _asbp_gm_main (cast `/Game/Blueprints/GameModes/BP_GM_Main` (`GameplayStatics.GetGameMode`)))
  (set `self.As BP GM Main` _asbp_gm_main)
  (bind _output_get (set `/Game/Blueprints/GameModes/BP_GM_Main.isPacking` (`self.Is Packing`) _asbp_gm_main))
  (if _output_get
    (bind _outactors (`GameplayStatics.GetAllActorsOfClass` "/Game/Blueprints/Furniture/BP_A_Furniture.BP_A_Furniture_C"))
    (for _array_element _outactors
      (`KismetArrayLibrary.Array_Add` _furnitures _array_element))
    (for _array_element_2 _furnitures
      (`/Game/Blueprints/Furniture/BP_A_Furniture.PopulateItems` _array_element_2))
    (bind _outactors_2 (`GameplayStatics.GetAllActorsOfClass` "/Game/Blueprints/Furniture/BP_A_Furniture.BP_A_Furniture_C"))
    (for _array_element_3 _outactors_2
      (for _array_element_4 (`/Game/Blueprints/Furniture/BP_A_Furniture.InItems` _array_element_3)
        (set `/Game/Blueprints/ItemInteractables/BP_A_ItemInteractable.isInFurniture` true _array_element_4)))
    (`/Game/Blueprints/GameModes/BP_GM_Main.GetAllItems` (`self.As BP GM Main`))
    (else
      (bind _outactors_3 (`GameplayStatics.GetAllActorsOfClass` "/Game/Blueprints/Box/BP_A_Package.BP_A_Package_C"))
      (for _array_element_5 _outactors_3
        (`KismetArrayLibrary.Array_Add` (`self.Packages`) _array_element_5))
      (for _array_element_6 (`self.Packages`)
        (`/Game/Blueprints/Box/BP_A_Package.PopulateItems` _array_element_6))
      (bind _outactors_4 (`GameplayStatics.GetAllActorsOfClass` "/Game/Blueprints/Box/BP_A_Package.BP_A_Package_C"))
      (for _array_element_7 _outactors_4
        (for _array_element_8 (`/Game/Blueprints/Box/BP_A_Package.InBox` _array_element_7)
          (set `/Game/Blueprints/ItemInteractables/BP_A_ItemInteractable.isPackaged` true _array_element_8)))
      (`/Game/Blueprints/GameModes/BP_GM_Main.GetAllItems` (`self.As BP GM Main`)))))

(fn `UserConstructionScript`)