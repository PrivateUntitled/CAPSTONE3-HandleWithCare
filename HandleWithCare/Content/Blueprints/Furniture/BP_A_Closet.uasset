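; BP_A_Closet is a two-door closet, a child of a furniture parent class, that holds hanging clothes and seven slot grids.
; The construction script spawns a BP_A_ClothesCloset part at HangedShirts and initializes the grids, which BeginPlay adds to GridStruct.
; Open and close events play separate timelines per door that lerp yaw, each stopping its opposite during updates.
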(event `self.ReceiveBeginPlay`
  (bind _gridstruct (`self.GridStruct`))
  (`parent.ReceiveBeginPlay`)
  (`KismetArrayLibrary.Array_Add` _gridstruct (make `/Game/Blueprints/Structure/GridStruct` (`self.Grids`)))
  (`KismetArrayLibrary.Array_Add` _gridstruct (make `/Game/Blueprints/Structure/GridStruct` (`self.Grids2`)))
  (`KismetArrayLibrary.Array_Add` _gridstruct (make `/Game/Blueprints/Structure/GridStruct` (`self.Grids3`)))
  (`KismetArrayLibrary.Array_Add` _gridstruct (make `/Game/Blueprints/Structure/GridStruct` (`self.Grids4`)))
  (`KismetArrayLibrary.Array_Add` _gridstruct (make `/Game/Blueprints/Structure/GridStruct` (`self.Grids5`)))
  (`KismetArrayLibrary.Array_Add` _gridstruct (make `/Game/Blueprints/Structure/GridStruct` (`self.Grids6`)))
  (`KismetArrayLibrary.Array_Add` _gridstruct (make `/Game/Blueprints/Structure/GridStruct` (`self.Grids7`))))

(event `self.OpenFurniture`
  (`parent.OpenFurniture`)
  (`|ExecutionSequence`
    (:`then_0`
      (bind (_direction _leftdooropen) (`Timeline|LeftDoorOpen` :!via `PlayFromStart` :!label _label)
        (:`Update`
          (`SceneComponent.K2_SetRelativeRotation` (`self.LeftDoor`) (`KismetMathLibrary.MakeRotator` 0.0 0.0 (`KismetMathLibrary.Lerp` (`self.LeftDoorCloseFloat`) (`self.LeftDoorOpenFloat`) _leftdooropen)) false false)
          (bind (_direction_2 _leftdooropen_2) (`Timeline|Timeline` :!via `Stop` :!label _label_2)
            (:`Update`
              (`SceneComponent.K2_SetRelativeRotation` (`self.LeftDoor`) (`KismetMathLibrary.MakeRotator` 0.0 0.0 (`KismetMathLibrary.Lerp` (`self.LeftDoorOpenFloat`) (`self.LeftDoorCloseFloat`) _leftdooropen_2)) false false)
              (goto _label :!via `Stop`))))))
    (:`then_1`
      (bind (_direction_3 _rightdooropen) (`Timeline|RightDoorOpen` :!via `PlayFromStart` :!label _label_3)
        (:`Update`
          (`SceneComponent.K2_SetRelativeRotation` (`self.RightDoor`) (`KismetMathLibrary.MakeRotator` 0.0 0.0 (`KismetMathLibrary.Lerp` (`self.RightDoorCloseFloat`) (`self.RightDoorOpenFloat`) _rightdooropen)) false false)
          (bind (_direction_4 _rightdooropen_2) (`Timeline|Timeline_0` :!via `Stop` :!label _label_4)
            (:`Update`
              (`SceneComponent.K2_SetRelativeRotation` (`self.RightDoor`) (`KismetMathLibrary.MakeRotator` 0.0 0.0 (`KismetMathLibrary.Lerp` (`self.RightDoorOpenFloat`) (`self.RightDoorCloseFloat`) _rightdooropen_2)) false false)
              (goto _label_3 :!via `Stop`))))))))

(event `self.OnFurnitureClose`
  (`parent.OnFurnitureClose`)
  (`|ExecutionSequence`
    (:`then_0`
      (goto _label_2 :!via `PlayFromStart`))
    (:`then_1`
      (goto _label_4 :!via `PlayFromStart`))))

(fn `UserConstructionScript`
  (`parent.UserConstructionScript`)
  (bind _child (`self.SpawnFurnitureParts` (`self.HangedShirts`) "/Game/Blueprints/Furniture/FurnitureParts/SwitchableItems/BP_A_ClothesCloset.BP_A_ClothesCloset_C"))
  (set `self.Shirts` _child)
  (`self.InitializeGrid` 7 2 (`self.Grid`) (`self.Grids`))
  (`self.InitializeGrid` 3 2 (`self.Grid2`) (`self.Grids2`))
  (`self.InitializeGrid` 3 2 (`self.Grid3`) (`self.Grids3`))
  (`self.InitializeGrid` 3 2 (`self.Grid4`) (`self.Grids4`))
  (`self.InitializeGrid` 3 2 (`self.Grid5`) (`self.Grids5`))
  (`self.InitializeGrid` 3 2 (`self.Grid6`) (`self.Grids6`))
  (`self.InitializeGrid` 3 2 (`self.Grid7`) (`self.Grids7`)))