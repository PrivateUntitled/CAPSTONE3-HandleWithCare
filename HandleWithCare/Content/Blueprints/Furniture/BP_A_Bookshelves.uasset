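; BP_A_Bookshelves is a bookshelf furniture actor with five slot grids, built on inherited parent setup.
; The construction script calls InitializeGrid for each Grid scene component, filling five separate arrays with an identical row and column layout.
; BeginPlay runs the parent logic, then adds all five arrays to GridStruct, gathering the grids into one collection.
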(event `self.ReceiveBeginPlay`
  (bind _gridstruct (`self.GridStruct`))
  (`parent.ReceiveBeginPlay`)
  (`KismetArrayLibrary.Array_Add` _gridstruct (make `/Game/Blueprints/Structure/GridStruct` (`self.Grids`)))
  (`KismetArrayLibrary.Array_Add` _gridstruct (make `/Game/Blueprints/Structure/GridStruct` (`self.Grids2`)))
  (`KismetArrayLibrary.Array_Add` _gridstruct (make `/Game/Blueprints/Structure/GridStruct` (`self.Grids3`)))
  (`KismetArrayLibrary.Array_Add` _gridstruct (make `/Game/Blueprints/Structure/GridStruct` (`self.Grids4`)))
  (`KismetArrayLibrary.Array_Add` _gridstruct (make `/Game/Blueprints/Structure/GridStruct` (`self.Grids5`))))

(fn `UserConstructionScript`
  (`parent.UserConstructionScript`)
  (`self.InitializeGrid` 2 7 (`self.Grid`) (`self.Grids`))
  (`self.InitializeGrid` 2 7 (`self.Grid2`) (`self.Grids2`))
  (`self.InitializeGrid` 2 7 (`self.Grid3`) (`self.Grids3`))
  (`self.InitializeGrid` 2 7 (`self.Grid4`) (`self.Grids4`))
  (`self.InitializeGrid` 2 7 (`self.Grid5`) (`self.Grids5`)))