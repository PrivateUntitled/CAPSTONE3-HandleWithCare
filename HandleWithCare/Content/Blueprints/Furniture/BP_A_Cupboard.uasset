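; Cupboard furniture actor with two swinging doors and four 2x2 grids, built on a parent furniture class.
; The construction script initializes each grid at its scene component, and BeginPlay registers the grids and two static meshes in arrays.
; Open and close events drive separate per-door timelines that lerp relative yaw between closed and open angles.
; Each timeline's update stops its opposite, so a new open or close interrupts the running motion.
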(event `self.ReceiveBeginPlay`
  (bind _staticmeshes (`self.StaticMeshes`))
  (bind _gridstruct (`self.GridStruct`))
  (`parent.ReceiveBeginPlay`)
  (`KismetArrayLibrary.Array_Add` _gridstruct (make `/Game/Blueprints/Structure/GridStruct` (`self.Grids1`)))
  (`KismetArrayLibrary.Array_Add` _gridstruct (make `/Game/Blueprints/Structure/GridStruct` (`self.Grids2`)))
  (`KismetArrayLibrary.Array_Add` _gridstruct (make `/Game/Blueprints/Structure/GridStruct` (`self.Grids3`)))
  (`KismetArrayLibrary.Array_Add` _gridstruct (make `/Game/Blueprints/Structure/GridStruct` (`self.Grids4`)))
  (`KismetArrayLibrary.Array_Add` _staticmeshes (`self.StaticMesh2`))
  (`KismetArrayLibrary.Array_Add` _staticmeshes (`self.StaticMesh1_0`)))

(event `self.OpenFurniture`
  (`parent.OpenFurniture`)
  (`|ExecutionSequence`
    (:`then_0`
      (bind (_direction _leftdooropen) (`Timeline|Timeline` :!via `PlayFromStart` :!label _label)
        (:`Update`
          (`SceneComponent.K2_SetRelativeRotation` (`self.LeftDoor`) (`KismetMathLibrary.MakeRotator` 0.0 0.0 (`KismetMathLibrary.Lerp` (`self.LeftDoorCloseFloat`) (`self.LeftDoorOpenFloat`) _leftdooropen)) false false)
          (bind (_direction_2 _leftdooropen_2) (`Timeline|Timeline_1` :!via `Stop` :!label _label_2)
            (:`Update`
              (`SceneComponent.K2_SetRelativeRotation` (`self.LeftDoor`) (`KismetMathLibrary.MakeRotator` 0.0 0.0 (`KismetMathLibrary.Lerp` (`self.LeftDoorOpenFloat`) (`self.LeftDoorCloseFloat`) _leftdooropen_2)) false false)
              (goto _label :!via `Stop`))))))
    (:`then_1`
      (bind (_direction_3 _rightdooropen) (`Timeline|Timeline_0` :!via `PlayFromStart` :!label _label_3)
        (:`Update`
          (`SceneComponent.K2_SetRelativeRotation` (`self.RightDoor`) (`KismetMathLibrary.MakeRotator` 0.0 0.0 (`KismetMathLibrary.Lerp` (`self.RightDoorCloseFloat`) (`self.RightDoorOpenFloat`) _rightdooropen)) false false)
          (bind (_direction_4 _rightdooropen_2) (`Timeline|Timeline_2` :!via `Stop` :!label _label_4)
            (:`Update`
              (`SceneComponent.K2_SetRelativeRotation` (`self.RightDoor`) (`KismetMathLibrary.MakeRotator` 0.0 0.0 (`KismetMathLibrary.Lerp` (`self.RightDoorOpenFloat`) (`self.RightDoorCloseFloat`) _rightdooropen_2)) false false)
              (goto _label_3 :!via `Stop`))))))))

(event `self.OnFurnitureClose`
  (`parent.OnFurnitureClose`)
  (`|ExecutionSequence`
    (:`then_0`
      (goto _label_2 :!via `PlayFromStart`))
    (:`then_1`
      (goto _label_4 :!via `PlayFromStart`))))

(fn `UserConstructionScript`
  (`parent.UserConstructionScript`)
  (`self.InitializeGrid` 2 2 (`self.Grid1`) (`self.Grids1`))
  (`self.InitializeGrid` 2 2 (`self.Grid2`) (`self.Grids2`))
  (`self.InitializeGrid` 2 2 (`self.Grid3`) (`self.Grids3`))
  (`self.InitializeGrid` 2 2 (`self.Grid4`) (`self.Grids4`)))