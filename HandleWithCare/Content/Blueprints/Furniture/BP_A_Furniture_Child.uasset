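; Furniture actor child Blueprint that gives its piece two grids of opposite proportions.
; The construction script runs the parent's setup, then calls InitializeGrid to fill a separate array from each of two grid scene components, one 3 by 6 and the other 6 by 3.
; BeginPlay calls the parent, then adds both arrays to GridStruct.
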(event `self.ReceiveBeginPlay`
  (`parent.ReceiveBeginPlay`)
  (`KismetArrayLibrary.Array_Add` (`self.GridStruct`) (make `/Game/Blueprints/Structure/GridStruct` (`self.Grids1`)))
  (`KismetArrayLibrary.Array_Add` (`self.GridStruct`) (make `/Game/Blueprints/Structure/GridStruct` (`self.Grids2`))))

(fn `UserConstructionScript`
  (`parent.UserConstructionScript`)
  (`self.InitializeGrid` 3 6 (`self.Grid1`) (`self.Grids1`))
  (`self.InitializeGrid` 6 3 (`self.Grid2`) (`self.Grids2`)))