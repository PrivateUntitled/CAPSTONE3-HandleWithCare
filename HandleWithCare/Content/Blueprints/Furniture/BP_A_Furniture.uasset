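; Base furniture actor that the player hovers to highlight and presses E to enter a close-up item-placement mode.
; Opening blends the camera to it, stacks carried items as draggable, hides the player, overlapping furniture and unstored packages, and shows UI and grids; closing restores surroundings.
; Helpers build child-actor grids and parts, return or drop leftover items, and pre-fill grids through a populate component.
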(event `self.ReceiveBeginPlay`
  (bind _asbp_third_person_character (cast `/Game/ThirdPerson/Blueprints/BP_ThirdPersonCharacter` (`GameplayStatics.GetPlayerPawn` 0)))
  (set `self.As BP Third Person Character` _asbp_third_person_character)
  (bind _returnvalue (`|GenericCreateObject` "/Game/Blueprints/Widgets/WB_FurnitureUI.WB_FurnitureUI_C"))
  (set `self.CategoryWidget` _returnvalue)
  (bind _returnvalue_2 (`|GenericCreateObject` "/Game/Blueprints/Player/PlayerUI/WB_BoxUI.WB_BoxUI_C"))
  (set `self.InteractWidget` _returnvalue_2)
  (`KismetArrayLibrary.Array_Add` (`self.StaticMeshes`) (`self.StaticMesh`))
  (add `self.OnOpenFurniture` (delegate `OnFurnitureOpen`))
  (add `self.OnCloseFurniture` (delegate `OnFurnitureClose`))
  (`KismetSystemLibrary.Delay` 0.2)
  (for _array_element (`PrimitiveComponent.GetOverlappingActors` (`self.SurroundingFurnitures`) "BP_A_Furniture_C")
    (bind _asbp_a_furniture (cast `/Game/Blueprints/Furniture/BP_A_Furniture` _array_element))
    (if (!= _asbp_a_furniture self)
      (`KismetArrayLibrary.Array_Add` (`self.OverlappingFurnitures`) _asbp_a_furniture)))
  (if (`KismetArrayLibrary.Array_IsNotEmpty` (`self.ItemsToPopulate`))
    (`self.PopulateItems`)))

(event `OnFurnitureOpen`
  (bind _categorywidget (`self.CategoryWidget`))
  ;[1 1 1] On Furniture Open
  (`self.CheckBoxes` true)
  (for _array_element (`self.OverlappingFurnitures`)
    (`self.SetActorHiddenInGame` _array_element true)
    (`self.SetActorEnableCollision` _array_element false)
    (for _array_element_2 (`/Game/Blueprints/Furniture/BP_A_Furniture.InItems` _array_element)
      (`/Engine/EditorBlueprintResources/StandardMacros.IsValid` _array_element_2
        (:`Is Valid`
          (`self.SetActorHiddenInGame` _array_element_2 true)))))
  (`UserWidget.AddToViewport` _categorywidget 0)
  (`/Game/Blueprints/Widgets/WB_FurnitureUI.SetCategoryDisplay` _categorywidget self)
  (for _array_element_3 (`self.GridStruct`) :!label _label
    (`self.ShowGrid` (break `/Game/Blueprints/Structure/GridStruct` _array_element_3))))

(event `OnFurnitureClose`
  ;[1 1 1] On Furniture Closed
  (`self.CheckBoxes` false true)
  (for _array_element (`self.OverlappingFurnitures`)
    (`self.SetActorHiddenInGame` _array_element false)
    (`self.SetActorEnableCollision` _array_element true)
    (for _array_element_2 (`/Game/Blueprints/Furniture/BP_A_Furniture.InItems` _array_element)
      (`/Engine/EditorBlueprintResources/StandardMacros.IsValid` _array_element_2
        (:`Is Valid`
          (`self.SetActorHiddenInGame` _array_element_2 false)))))
  (`Widget.RemoveFromParent` (`self.CategoryWidget`))
  (goto _label))

(event `self.BoxCollision.OnBeginCursorOver`
  (params (TouchedComponent :type "PrimitiveComponent Object Reference"))
  (bind _as_bp_third_person_character (`self.As BP Third Person Character`))
  ;[1 1 1] On Cursor Hover/Unhover
  (if (`self.IsEnabled`)
    (`self.On Hover`)
    (if (not (`/Game/ThirdPerson/Blueprints/BP_ThirdPersonCharacter.IsInteracting` _as_bp_third_person_character))
      (`self.EnableInput` (`/Game/ThirdPerson/Blueprints/BP_ThirdPersonCharacter.As BP Player Controller` _as_bp_third_person_character)))))

(event `self.BoxCollision.OnEndCursorOver`
  (params (TouchedComponent :type "PrimitiveComponent Object Reference"))
  ;[1 1 1] On Cursor Hover/Unhover
  (if (`self.IsEnabled`)
    (`self.OnUnhover`)
    (if (not (`/Game/ThirdPerson/Blueprints/BP_ThirdPersonCharacter.IsInteracting` (`self.As BP Third Person Character`)))
      (`self.DisableInput` (`/Game/ThirdPerson/Blueprints/BP_ThirdPersonCharacter.As BP Player Controller` (`self.As BP Third Person Character`))))))

(event `Key|E`
  (params (Key :type "Key Structure"))
  (bind _as_bp_third_person_character (`self.As BP Third Person Character`))
  (bind _items (`/Game/ThirdPerson/Blueprints/BP_ThirdPersonCharacter.Items` (`self.As BP Third Person Character`)))
  ;[1 1 1] E to Pickup
  (:`Pressed`
    (if (`/Game/ThirdPerson/Blueprints/BP_ThirdPersonCharacter.IsInteracting` _as_bp_third_person_character)
      _
      (elif (not (`KismetSystemLibrary.DoesImplementInterface` (`|GetArrayItem` (`/Game/ThirdPerson/Blueprints/BP_ThirdPersonCharacter.Items` _as_bp_third_person_character)) "/Game/Blueprints/ItemInteractables/BlueprintInterface/BI_Openable.BI_Openable_C"))
        (`self.ChangeCamera`)
        (`self.GetItems` (`self.ItemInitialLocation`) _items)
        (for _array_element _items
          (`PrimitiveComponent.SetCollisionResponseToChannel` (`/Game/Blueprints/ItemInteractables/BP_A_ItemInteractable.Collision` _array_element) "ECC_Visibility" "ECR_Block"))
        (`self.OpenFurniture`)))))

(event `OpenFurniture`
  (bind _as_bp_third_person_character (`self.As BP Third Person Character`))
  (bind _as_bp_player_controller (`/Game/ThirdPerson/Blueprints/BP_ThirdPersonCharacter.As BP Player Controller` _as_bp_third_person_character))
  (bind _items (`/Game/ThirdPerson/Blueprints/BP_ThirdPersonCharacter.Items` (`self.As BP Third Person Character`)))
  ;[1 1 1] Open Furniture
  (set `/Game/ThirdPerson/Blueprints/BP_ThirdPersonCharacter.CurrentFurniture` self (`self.As BP Third Person Character`))
  (set `/Game/ThirdPerson/Blueprints/BP_ThirdPersonCharacter.IsInteracting` true (`self.As BP Third Person Character`))
  (`UserWidget.AddToViewport` (`self.InteractWidget`) 0)
  (for _array_element _items
    (set `/Game/Blueprints/ItemInteractables/BP_A_ItemInteractable.canBeDragged` true _array_element))
  (set `self.OutItems` _items)
  (`KismetArrayLibrary.Array_Clear` _items)
  (for _array_element_2 (`self.InItems`)
    (`/Engine/EditorBlueprintResources/StandardMacros.IsValid` _array_element_2
      (:`Is Valid`
        (`PrimitiveComponent.SetCollisionEnabled` (`/Game/Blueprints/ItemInteractables/BP_A_ItemInteractable.Collision` _array_element_2) "QueryAndPhysics"))))
  (`PrimitiveComponent.SetCollisionResponseToChannel` (`self.BoxCollision`) "ECC_Visibility" "ECR_Ignore")
  (`self.SetActorHiddenInGame` (`self.As BP Third Person Character`) true)
  (`self.OnOpenFurniture`)
  (`self.DisableInput` _as_bp_third_person_character _as_bp_player_controller)
  (`self.DisableInput` _as_bp_player_controller)
  (`/Game/ThirdPerson/Blueprints/BP_ThirdPersonCharacter.CheckItemCategory` (`self.As BP Third Person Character`)))

(fn `ChangeCamera`
  (bind _as_bp_third_person_character (`self.As BP Third Person Character`))
  (`PlayerController.SetViewTargetWithBlend` (`/Game/ThirdPerson/Blueprints/BP_ThirdPersonCharacter.As BP Player Controller` (`self.As BP Third Person Character`)) self 0.0 "VTBlend_Linear" 0.0 false)
  (set `/Game/ThirdPerson/Blueprints/BP_ThirdPersonCharacter.IsInteracting` true _as_bp_third_person_character)
  (set `/Game/ThirdPerson/Blueprints/BP_ThirdPersonCharacter.HasHoveredItem` false _as_bp_third_person_character)
  (`/Game/Blueprints/Player/BP_PlayerController.SetMouse` (`/Game/ThirdPerson/Blueprints/BP_ThirdPersonCharacter.As BP Player Controller` _as_bp_third_person_character) false true))

(fn `CheckBoxes`
  (params (bNewHidden :type Boolean) (bNewActorEnableCollision :type Boolean))
  (bind _outactors (`GameplayStatics.GetAllActorsOfClass` "/Game/Blueprints/Box/BP_A_Package.BP_A_Package_C"))
  (if (`KismetArrayLibrary.Array_IsValidIndex` _outactors)
    (for _array_element _outactors
      (if (not (`/Game/Blueprints/Box/BP_A_Package.isStored` _array_element))
        (`self.SetActorHiddenInGame` _array_element bNewHidden)
        (`self.SetActorEnableCollision` _array_element bNewActorEnableCollision)
        (`PrimitiveComponent.SetSimulatePhysics` (`/Game/Blueprints/ItemInteractables/BP_A_ItemInteractable.Collision` _array_element) bNewActorEnableCollision)
        (`KismetSystemLibrary.PrintString` (`KismetSystemLibrary.GetDisplayName` _array_element))
        (for _array_element_2 (`/Game/Blueprints/Box/BP_A_Package.InBox` _array_element)
          (`/Engine/EditorBlueprintResources/StandardMacros.IsValid` _array_element_2
            (:`Is Valid`
              (`self.SetActorHiddenInGame` _array_element_2 bNewHidden)
              (`self.SetActorEnableCollision` _array_element_2 bNewActorEnableCollision))))))))

(fn `CheckCorrectItems`
  (for _array_element (`self.InItems`)
    (if (`KismetArrayLibrary.Array_Contains` (`self.AllowedItemCategories`) (`/Game/Blueprints/ItemInteractables/BP_A_ItemInteractable.ItemCategory` _array_element))
      _)))

(fn `ClearGrid`
  (params (Grids :type "Array of /Game/Blueprints/Box/Grids/BP_A_Grid Object Reference"))
  (if (> (`KismetArrayLibrary.Array_Length` Grids) 0)
    (bind (_arrayindex _arrayelement) (`/Engine/EditorBlueprintResources/StandardMacros.ReverseForEachLoop` Grids)
      (:`LoopBody`
        (`/Engine/EditorBlueprintResources/StandardMacros.IsValid` _arrayelement
          (:`Is Valid`
            (`self.K2_DestroyActor` _arrayelement))))
      (:`Completed`
        (`KismetArrayLibrary.Array_Clear` Grids)))))

(fn `DropOutItems`
  (bind _outitems (`self.OutItems`))
  (for _array_element (`self.OutItems`)
    (set `/Game/Blueprints/ItemInteractables/BP_A_ItemInteractable.isInFurniture` false _array_element)
    (set `/Game/Blueprints/ItemInteractables/BP_A_ItemInteractable.canBeDragged` false _array_element)
    (`self.K2_SetActorLocation` _array_element (`SceneComponent.K2_GetComponentLocation` (`self.DropLocation`)) false false)
    (bind _collision (`/Game/Blueprints/ItemInteractables/BP_A_ItemInteractable.Collision` _array_element))
    (`PrimitiveComponent.SetConstraintMode` _collision "Default")
    (`self.K2_DetachFromActor` _array_element "KeepWorld" "KeepWorld" "KeepWorld")
    (`PrimitiveComponent.SetSimulatePhysics` _collision true)
    (bind _collision_2 (`/Game/Blueprints/ItemInteractables/BP_A_ItemInteractable.Collision` _array_element))
    (`PrimitiveComponent.SetCollisionResponseToChannel` _collision_2 "ECC_Visibility" "ECR_Block")
    (`PrimitiveComponent.SetCollisionEnabled` _collision_2 "QueryAndPhysics"))
  (for _array_element_2 _outitems
    (`KismetArrayLibrary.Array_RemoveItem` _outitems _array_element_2)))

(fn `GetItems`
  (params (`Scene Component` :type "SceneComponent Object Reference") (Items :type "Array of /Game/Blueprints/ItemInteractables/BP_A_ItemInteractable Object Reference"))
  (for (_array_element _array_index) Items
    (if (== _array_index 0)
      (`self.K2_DetachFromActor` _array_element "KeepWorld" "KeepWorld" "KeepWorld")
      (`self.K2_SetActorLocation` _array_element (`SceneComponent.K2_GetComponentLocation` `Scene Component`) false false)
      (`self.K2_SetActorRotation` _array_element (`SceneComponent.K2_GetComponentRotation` `Scene Component`) false)
      (`/Game/Blueprints/ItemInteractables/BP_A_ItemInteractable.PlayAssignedDialogue` _array_element)
      (else
        (bind _output (`|GetArrayItem` Items _array_index))
        (`self.K2_DetachFromActor` _output "KeepWorld" "KeepWorld" "KeepWorld")
        (bind (_origin _boxextent) (`KismetSystemLibrary.GetComponentBounds` (`/Game/Blueprints/ItemInteractables/BP_A_ItemInteractable.StaticMesh` (`|GetArrayItem` Items (- _array_index 1)))))
        (`self.K2_SetActorLocation` _output (`KismetMathLibrary.MakeVector` (.x _origin) (.y _origin) (+ (.z _origin) (* (.z _boxextent) 2.0))) false false)
        (`self.K2_SetActorRotation` _output (`SceneComponent.K2_GetComponentRotation` `Scene Component`) false)
        (`/Game/Blueprints/ItemInteractables/BP_A_ItemInteractable.PlayAssignedDialogue` _array_element)))))

(fn `GetOutItems`
  (bind _outitems (`self.OutItems`))
  (bind _as_bp_third_person_character (`self.As BP Third Person Character`))
  (bind _outitems_2 (`self.OutItems`))
  (bind _itemplacement (`/Game/ThirdPerson/Blueprints/BP_ThirdPersonCharacter.ItemPlacement` _as_bp_third_person_character))
  (`self.GetItems` _itemplacement _outitems)
  (for _array_element _outitems
    (`self.K2_AttachToComponent` _array_element _itemplacement "None" "KeepWorld" "KeepWorld" "KeepWorld" true)
    (bind _collision (`/Game/Blueprints/ItemInteractables/BP_A_ItemInteractable.Collision` _array_element))
    (`PrimitiveComponent.SetCollisionResponseToChannel` _collision "ECC_Visibility" "ECR_Ignore")
    (`PrimitiveComponent.SetCollisionEnabled` (`/Game/Blueprints/ItemInteractables/BP_A_ItemInteractable.StaticMesh` _array_element) "PhysicsOnly")
    (`self.K2_SetActorRotation` _array_element (`self.K2_GetActorRotation` (`self.As BP Third Person Character`)) false)
    (`PrimitiveComponent.SetConstraintMode` _collision "None"))
  (set `/Game/ThirdPerson/Blueprints/BP_ThirdPersonCharacter.Items` _outitems_2 _as_bp_third_person_character)
  (`KismetArrayLibrary.Array_Clear` _outitems_2)
  (`/Game/ThirdPerson/Blueprints/BP_ThirdPersonCharacter.CheckItemCategory` (`self.As BP Third Person Character`)))

(fn `InitializeGrid`
  (params (Rows :type Integer) (Columns :type Integer) (`Scene Component` :type "SceneComponent Object Reference") (TargetArray :type "Array of /Game/Blueprints/Box/Grids/BP_A_Grid Object Reference (by ref)") (AddToGridLength :type "Float (double-precision)"))
  (bind _gridlength (`self.GridLength`))
  (`self.ClearGrid` TargetArray)
  (for _index (range Rows)
    (for _index_2 (range Columns)
      (bind _returnvalue (`AddComponent|NODE_AddChildActorComponent-0` :`RelativeTransform` (`KismetMathLibrary.MakeTransform` (`self.K2_GetActorLocation`) (`self.K2_GetActorRotation`))))
      (`ChildActorComponent.SetChildActorClass` _returnvalue (`self.GridType`))
      (bind _asbp_a_grid (cast `/Game/Blueprints/Box/Grids/BP_A_Grid` (`ChildActorComponent.ChildActor` _returnvalue)))
      (`self.SetOwner` _asbp_a_grid self)
      (bind _box (`/Game/Blueprints/Box/Grids/BP_A_Grid.Box` _asbp_a_grid))
      (`BoxComponent.SetBoxExtent` _box (`KismetMathLibrary.MakeVector` 40.0 40.0 (+ AddToGridLength _gridlength)) true)
      (`SceneComponent.K2_SetRelativeLocation` _box (`KismetMathLibrary.MakeVector` 0.0 0.0 (+ AddToGridLength _gridlength)) false false)
      (set `/Game/Blueprints/Box/Grids/BP_A_Grid.Row` _index _asbp_a_grid)
      (set `/Game/Blueprints/Box/Grids/BP_A_Grid.Column` _index_2 _asbp_a_grid)
      (set `/Game/Blueprints/Box/Grids/BP_A_Grid.GridCellSize` (`self.GridCellSize`) _asbp_a_grid)
      (`/Game/Blueprints/Box/Grids/BP_A_Grid.Initialize` _asbp_a_grid `Scene Component`)
      (`/Game/Blueprints/Box/Grids/BP_A_Grid.GetPositionXY` _asbp_a_grid)
      (`KismetArrayLibrary.Array_AddUnique` TargetArray _asbp_a_grid))))

(fn `On Hover`
  (bind _as_bp_third_person_character (`self.As BP Third Person Character`))
  (if (not (`/Game/ThirdPerson/Blueprints/BP_ThirdPersonCharacter.IsInteracting` (`self.As BP Third Person Character`)))
    (set `/Game/ThirdPerson/Blueprints/BP_ThirdPersonCharacter.CurrentHoveredFurniture` self _as_bp_third_person_character)
    (`KismetSystemLibrary.PrintString` (`KismetSystemLibrary.GetDisplayName` self))
    (set `/Game/ThirdPerson/Blueprints/BP_ThirdPersonCharacter.HasHoveredItem` true _as_bp_third_person_character)
    (for _array_element (`self.StaticMeshes`)
      (for (_ _array_index) (`MeshComponent.GetMaterials` _array_element)
        (`PrimitiveComponent.SetMaterial` _array_element _array_index "/Game/Blueprints/Materials/Highlight.Highlight")))))

(fn `OnUnhover`
  (bind _as_bp_third_person_character (`self.As BP Third Person Character`))
  (set `/Game/ThirdPerson/Blueprints/BP_ThirdPersonCharacter.CurrentHoveredFurniture` null _as_bp_third_person_character)
  (set `/Game/ThirdPerson/Blueprints/BP_ThirdPersonCharacter.HasHoveredItem` false _as_bp_third_person_character)
  (for _array_element (`self.StaticMeshes`)
    (for (_ _array_index) (`MeshComponent.GetMaterials` _array_element)
      (`PrimitiveComponent.SetMaterial` _array_element _array_index (`self.OriginalMaterial`)))))

(fn `PopulateItems`
  (bind _itemstopopulate (`self.ItemsToPopulate`))
  (if (`KismetArrayLibrary.Array_IsValidIndex` _itemstopopulate)
    (for (_array_element _array_index) _itemstopopulate
      (for _array_element_2 (`/Game/Blueprints/DataAssets/PopulateItemsDataAssets/DA_PopulateItems.PopulateItemsStruct` _array_element)
        (bind _output_grid (break `/Game/Blueprints/Structure/GridStruct` (`|GetArrayItem` (`self.GridStruct`) _array_index)))
        (`/Game/Blueprints/Player/BP_AC_PopulateItems.PopulateItems` (`self.BP_AC_PopulateItems`) _output_grid (break `/Game/Blueprints/Structure/PopulateItemsStruct` _array_element_2) (`.InitialColumn_12_08EABF644FC0E26138F02B9625A10D3A` (break `/Game/Blueprints/Structure/PopulateItemsStruct` _array_element_2)) (`.EndRow_14_7A8B15EE445E8A2B1BB91BA963DD0099` (break `/Game/Blueprints/Structure/PopulateItemsStruct` _array_element_2)) (`.EndColumn_16_2CEB51A9439026185000C7BC82E190C3` (break `/Game/Blueprints/Structure/PopulateItemsStruct` _array_element_2)) (`.Rotation_19_CBE0018B421A55AA5758EEA9B1EBAAAD` (break `/Game/Blueprints/Structure/PopulateItemsStruct` _array_element_2)) (`.Item_22_A1880C41486790E2DAEA9D81E4BCEC38` (break `/Game/Blueprints/Structure/PopulateItemsStruct` _array_element_2)) (`.NumberOfItems_25_21A11A934D797545D7F408A99A6CAEC9` (break `/Game/Blueprints/Structure/PopulateItemsStruct` _array_element_2)) self (`self.InItems`))))))

(fn `ShowGrid`
  (params (Array :type "Array of /Game/Blueprints/Box/Grids/BP_A_Grid Object Reference"))
  (for _array_element Array
    (`/Engine/EditorBlueprintResources/StandardMacros.IsValid` _array_element
      (:`Is Valid`
        (bind _grid (`/Game/Blueprints/Box/Grids/BP_A_Grid.Grid` _array_element))
        (if (`SceneComponent.bHiddenInGame` _grid)
          (`SceneComponent.SetHiddenInGame` _grid false false)
          (bind _box (`/Game/Blueprints/Box/Grids/BP_A_Grid.Box` _array_element))
          (`PrimitiveComponent.SetCollisionEnabled` _box "QueryOnly")
          (`PrimitiveComponent.SetCollisionResponseToChannel` _grid "ECC_Visibility" "ECR_Block")
          (else
            (`SceneComponent.SetHiddenInGame` _grid true false)
            (`PrimitiveComponent.SetCollisionEnabled` _box "NoCollision")
            (`PrimitiveComponent.SetCollisionResponseToChannel` _grid "ECC_Visibility" "ECR_Ignore")))))))

(fn `SpawnFurnitureParts`
  (params (Target :type "StaticMeshComponent Object Reference") (InClass :type "Actor Class Reference"))
  (returns (Child :type "Array of Actor Object Reference"))
  (bind _furniturepartschild (`self.FurniturePartsChild`))
  (for _array_element (`SceneComponent.GetChildrenComponents` Target false)
    (bind _returnvalue (`AddComponent|NODE_AddChildActorComponent-1` :`RelativeTransform` (`KismetMathLibrary.MakeTransform` (`SceneComponent.K2_GetComponentLocation` _array_element))))
    (`ChildActorComponent.SetChildActorClass` _returnvalue InClass)
    (`SceneComponent.K2_AttachToComponent` _returnvalue _array_element "None" "SnapToTarget" "SnapToTarget" "KeepWorld" true)
    (bind _childactor (`ChildActorComponent.ChildActor` _returnvalue))
    (`self.SetOwner` _childactor self)
    (`KismetArrayLibrary.Array_Add` _furniturepartschild _childactor))
  (return _furniturepartschild))

(fn `UserConstructionScript`)