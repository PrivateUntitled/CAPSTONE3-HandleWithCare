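; An actor component that detects interactable items the player looks at.
; It caches the player's ThirdPersonCharacter on BeginPlay, then line traces every Tick along the camera's forward vector on the Visibility channel, up to an interaction distance.
; Hit actors implementing BI_Item_Interactable receive InteractMessage each frame.
; A trace that hits nothing prints "no item" and clears the character's CurrentHoveredItem, while non-interactable hits leave it unchanged.
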(event `self.ReceiveBeginPlay`
  (bind _asbp_third_person_character (cast `/Game/ThirdPerson/Blueprints/BP_ThirdPersonCharacter` (`GameplayStatics.GetPlayerPawn` 0)))
  (set `self.As BP Third Person Character` _asbp_third_person_character))

(event `self.ReceiveTick`
  (params (DeltaSeconds :type "Float (single-precision)"))
  (bind _camera (`self.Camera`))
  (bind _returnvalue (`SceneComponent.K2_GetComponentLocation` _camera))
  (bind (_outhit _returnvalue_2) (`KismetSystemLibrary.LineTraceSingle` _returnvalue (+ _returnvalue (* (`SceneComponent.GetForwardVector` _camera) (`self.InteractionDistance`))) "TraceTypeQuery1"))
  (if _returnvalue_2
    (bind (_bblockinghit _binitialoverlap _time _distance _location _impactpoint _normal _impactnormal _physmat _hitactor) (`GameplayStatics.BreakHitResult` _outhit))
    (if (`KismetSystemLibrary.DoesImplementInterface` _hitactor "/Game/Blueprints/ItemInteractables/BI_Item_Interactable.BI_Item_Interactable_C")
      (message `/Game/Blueprints/ItemInteractables/BI_Item_Interactable.Interact` _hitactor))
    (else
      (`KismetSystemLibrary.PrintString` "no item")
      (set `/Game/ThirdPerson/Blueprints/BP_ThirdPersonCharacter.CurrentHoveredItem` null (`self.As BP Third Person Character`)))))