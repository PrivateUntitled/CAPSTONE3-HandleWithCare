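; Player pickup component that attaches the hovered item to the third-person character's ItemPlacement on left mouse click.
; Capacity comes from a MaxStackItem data asset, read through the GameInstance's TruckSpeed upgrade level.
; The first item triggers sound, dialogue and its pickup callback; later ones must match ItemNameID, with the held top item stackable, and sit atop it using mesh bounds.
; Pickups update carried weight, except the separate PickUpBox event, which attaches CurrentBox without checks.
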(event `self.ReceiveBeginPlay`
  (bind _asbp_third_person_character (cast `/Game/ThirdPerson/Blueprints/BP_ThirdPersonCharacter` (`GameplayStatics.GetPlayerPawn` 0)))
  (set `self.As BP Third Person Character` _asbp_third_person_character))

(event `Key|LeftMouseButton`
  (params (Key :type "Key Structure"))
  (:`Pressed`
    (`self.PickupItem`)))

(event `PickupItem`
  (bind _as_bp_third_person_character (`self.As BP Third Person Character`))
  (bind _items (`/Game/ThirdPerson/Blueprints/BP_ThirdPersonCharacter.Items` (`self.As BP Third Person Character`)))
  (bind _currenthovereditem (`/Game/ThirdPerson/Blueprints/BP_ThirdPersonCharacter.CurrentHoveredItem` _as_bp_third_person_character))
  (bind _currenthovereditem_2 (`/Game/ThirdPerson/Blueprints/BP_ThirdPersonCharacter.CurrentHoveredItem` (`self.As BP Third Person Character`)))
  (bind _items_2 (`/Game/ThirdPerson/Blueprints/BP_ThirdPersonCharacter.Items` (`self.As BP Third Person Character`)))
  (bind _itemplacement (`/Game/ThirdPerson/Blueprints/BP_ThirdPersonCharacter.ItemPlacement` _as_bp_third_person_character))
  (bind _items_3 (`/Game/ThirdPerson/Blueprints/BP_ThirdPersonCharacter.Items` (`self.As BP Third Person Character`)))
  (bind _returnvalue (`KismetArrayLibrary.Array_Length` (`/Game/ThirdPerson/Blueprints/BP_ThirdPersonCharacter.Items` _as_bp_third_person_character)))
  (bind _output (`|GetArrayItem` _items_2 (`KismetArrayLibrary.Array_LastIndex` _items_2)))
  (bind _collision (`/Game/Blueprints/ItemInteractables/BP_A_ItemInteractable.Collision` (`|GetArrayItem` _items (`KismetArrayLibrary.Array_LastIndex` _items))))
  (bind (_origin _boxextent) (`KismetSystemLibrary.GetComponentBounds` (`/Game/Blueprints/ItemInteractables/BP_A_ItemInteractable.StaticMesh` _output)))
  (bind _asbp_game_instance (cast `/Game/GameInstance/BP_GameInstance` (`GameplayStatics.GetGameInstance`)))
  (bind (_upgradedataasset _level) (break `/Game/GameInstance/Upgrades/UpgradeLevels` (`.TruckSpeed_6_68DE28D74222A81BD0480FA7EA87C0FC` (break `/Game/GameInstance/Upgrades/UpgradeList` (`/Game/GameInstance/BP_GameInstance.PlayerUpgrades` _asbp_game_instance)))))
  (bind _aspda_max_stack_item (cast `/Game/GameInstance/Upgrades/PDA_MaxStackItem` _upgradedataasset))
  (`/Engine/EditorBlueprintResources/StandardMacros.IsValid` _currenthovereditem
    (:`Is Valid`
      (if (< _returnvalue (`|GetArrayItem` (`/Game/GameInstance/Upgrades/PDA_MaxStackItem.MaxStackItem` _aspda_max_stack_item) _level))
        (if (> _returnvalue 0)
          (if (`KismetTextLibrary.EqualEqual_TextText` (`/Game/Blueprints/ItemInteractables/BP_A_ItemInteractable.ItemNameID` _output) (`/Game/Blueprints/ItemInteractables/BP_A_ItemInteractable.ItemNameID` _currenthovereditem))
            (if (`KismetSystemLibrary.DoesImplementInterface` _output "/Game/Blueprints/ItemInteractables/BlueprintInterface/BI_Item_Stackable.BI_Item_Stackable_C")
              (`Actor.K2_AttachToComponent` _currenthovereditem_2 (`/Game/ThirdPerson/Blueprints/BP_ThirdPersonCharacter.ItemPlacement` (`self.As BP Third Person Character`)) "None" "KeepWorld" "KeepWorld" "KeepWorld" true)
              (`Actor.K2_SetActorLocation` _currenthovereditem_2 (`KismetMathLibrary.MakeVector` (.x _origin) (.y _origin) (+ (.z _origin) (* (.z _boxextent) 2.0))) false false)
              (`Actor.K2_SetActorRotation` _currenthovereditem_2 (`Actor.K2_GetActorRotation` _output) false)
              (`PrimitiveComponent.SetSimulatePhysics` (`/Game/Blueprints/ItemInteractables/BP_A_ItemInteractable.Collision` _currenthovereditem_2) false)
              (`KismetArrayLibrary.Array_AddUnique` _items _currenthovereditem_2)
              (`PrimitiveComponent.SetCollisionResponseToChannel` _collision "ECC_Pawn" "ECR_Ignore")
              (`PrimitiveComponent.SetCollisionResponseToChannel` _collision "ECC_Visibility" "ECR_Ignore")
              (`/Game/ThirdPerson/Blueprints/BP_ThirdPersonCharacter.CalculateWeight` (`self.As BP Third Person Character`))))
          (else
            (`PrimitiveComponent.SetSimulatePhysics` (`/Game/Blueprints/ItemInteractables/BP_A_ItemInteractable.Collision` _currenthovereditem) false)
            (`KismetSystemLibrary.PrintString` (`KismetSystemLibrary.GetDisplayName` _currenthovereditem))
            (`Actor.K2_AttachToComponent` _currenthovereditem _itemplacement "None" "KeepWorld" "KeepWorld" "KeepWorld" true)
            (`Actor.K2_SetActorLocation` _currenthovereditem (`SceneComponent.K2_GetComponentLocation` _itemplacement) false false)
            (if (`KismetSystemLibrary.DoesImplementInterface` _currenthovereditem "/Game/Blueprints/ItemInteractables/BlueprintInterface/BI_Item_Stackable.BI_Item_Stackable_C")
              (`Actor.K2_SetActorRotation` _currenthovereditem (`KismetMathLibrary.ComposeRotators` (`SceneComponent.K2_GetComponentRotation` _itemplacement) (struct :`Yaw` 90.0)) false)
              (else
                (`Actor.K2_SetActorRelativeRotation` _currenthovereditem (`/Game/Blueprints/ItemInteractables/BP_A_ItemInteractable.ItemInitialRotation` _currenthovereditem) false false)))
            (`KismetArrayLibrary.Array_AddUnique` _items_3 _currenthovereditem)
            (`PrimitiveComponent.SetCollisionResponseToChannel` (`/Game/Blueprints/ItemInteractables/BP_A_ItemInteractable.Collision` (`|GetArrayItem` _items_3)) "ECC_Visibility" "ECR_Ignore")
            (`/Game/ThirdPerson/Blueprints/BP_ThirdPersonCharacter.CalculateWeight` (`self.As BP Third Person Character`))
            (`KismetSystemLibrary.PrintString` "PICKED UP")
            (`/Game/Blueprints/ItemInteractables/BP_A_ItemInteractable.itemPickedUp` _currenthovereditem)
            (`GameplayStatics.PlaySound2D` "/Game/SOUND_DESIGN/SFX/SFX_PickUp.SFX_PickUp" 1.0 1.0 0.0 null null)
            (`/Game/Blueprints/ItemInteractables/BP_A_ItemInteractable.PlayAssignedDialogue` (`/Game/ThirdPerson/Blueprints/BP_ThirdPersonCharacter.CurrentHoveredItem` (`self.As BP Third Person Character`)))))))))

(event `PickUpBox`
  (bind _as_bp_third_person_character (`self.As BP Third Person Character`))
  (bind _currentbox (`/Game/ThirdPerson/Blueprints/BP_ThirdPersonCharacter.CurrentBox` _as_bp_third_person_character))
  (bind _itemplacement (`/Game/ThirdPerson/Blueprints/BP_ThirdPersonCharacter.ItemPlacement` _as_bp_third_person_character))
  (bind _collision (`/Game/Blueprints/ItemInteractables/BP_A_ItemInteractable.Collision` _currentbox))
  (`PrimitiveComponent.SetSimulatePhysics` _collision false)
  (`Actor.K2_AttachToComponent` _currentbox _itemplacement "None" "KeepWorld" "KeepWorld" "KeepWorld" true)
  (`Actor.K2_SetActorLocation` _currentbox (`SceneComponent.K2_GetComponentLocation` _itemplacement) false false)
  (`PrimitiveComponent.SetCollisionEnabled` _collision "NoCollision")
  (`KismetArrayLibrary.Array_Add` (`/Game/ThirdPerson/Blueprints/BP_ThirdPersonCharacter.Items` (`self.As BP Third Person Character`)) _currentbox))