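; Actor component that spawns stackable items onto grid cells and rebuilds saved boxes with their contents.
; PopulateItems filters cells by row and column range, spawns the first item at their averaged center, then chains further items from the previous one's Arrow.
; Items attach to the first cell with collision disabled and share a stack owner, while cells are marked occupied and turned red.
; PopulateSavedItems spawns each box from saved package structs and attaches its items relatively.
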(fn `Populate Saved Items`
  (params (PackageStruct :type "Array of /Game/Blueprints/Structure/PackageStruct Structure") (BoxSpawnLocation :type "Array of Vector Structure") (Rotation :type "Array of Rotator Structure"))
  (for (_array_element _array_index) PackageStruct
    (bind _returnvalue (`|SpawnActorFromClass` (break `/Game/Blueprints/Structure/PackageStruct` _array_element) (`KismetMathLibrary.MakeTransform` (`|GetArrayItem` BoxSpawnLocation _array_index) (`|GetArrayItem` Rotation _array_index)) "Undefined" "MultiplyWithRoot" null null))
    (for _array_element_2 (`.ItemStruct_27_FD7B7C76463B1372BA6C239951008261` (break `/Game/Blueprints/Structure/PackageStruct` _array_element))
      (bind _returnvalue_2 (`|SpawnActorFromClass` (break `/Game/Blueprints/Structure/ItemStruct` _array_element_2) (`KismetMathLibrary.MakeTransform` (`.Location_6_E6A949BB445CB969F790878C051740C6` (break `/Game/Blueprints/Structure/ItemStruct` _array_element_2)) (`.Rotation_9_F1B159DE4DBA65746B89F99085B07607` (break `/Game/Blueprints/Structure/ItemStruct` _array_element_2))) "Undefined" "MultiplyWithRoot" null null))
      (`Actor.K2_AttachToActor` _returnvalue_2 _returnvalue "None" "KeepRelative" "KeepRelative" "KeepRelative" true)
      (`KismetArrayLibrary.Array_AddUnique` (`/Game/Blueprints/Box/BP_A_Package.InBox` _returnvalue) _returnvalue_2))))

(fn `PopulateItem`)

(fn `PopulateItems`
  (params (Grid :type "Array of /Game/Blueprints/Box/Grids/BP_A_Grid Object Reference") (InitialRow :type Integer) (InitialColumn :type Integer) (EndRow :type Integer) (EndColumn :type Integer) (Rotation :type "Rotator Structure") (Item :type "/Game/Blueprints/ItemInteractables/BP_A_ItemInteractable Class Reference") (NumberOfItems :type Integer) (ActorAttached :type "Actor Object Reference") (InItems :type "Array of Actor Object Reference"))
  (locals (`Filtrered Grid` :type "Array of /Game/Blueprints/Box/Grids/BP_A_Grid Object Reference") (SumOfGridLocations :type "Vector Structure") (MiddleLocation :type "Vector Structure") (Items :type "Array of /Game/Blueprints/ItemInteractables/BP_A_ItemInteractable Object Reference"))
  (bind _filtrered_grid (`local.Filtrered Grid`))
  (bind _items (`local.Items`))
  (bind _arrow (`/Game/Blueprints/ItemInteractables/BP_A_ItemInteractable.Arrow` (`|GetArrayItem` _items (`KismetArrayLibrary.Array_LastIndex` _items))))
  (bind _returnvalue (`SceneComponent.K2_GetComponentLocation` _arrow))
  ;[1 1 1] Get the chosen grids only
  (for _array_element Grid
    (bind _column (`/Game/Blueprints/Box/Grids/BP_A_Grid.Column` _array_element))
    (bind _row (`/Game/Blueprints/Box/Grids/BP_A_Grid.Row` _array_element))
    (if (and (>= _column InitialColumn) (<= _column EndColumn) (>= _row InitialRow) (<= _row EndRow))
      (`KismetArrayLibrary.Array_Add` _filtrered_grid _array_element)))
  ;[1 1 1] Getting the middle locations to spawn actors
  (for _array_element_2 _filtrered_grid
    (bind _output_get (set `local.SumOfGridLocations` (+ (`Actor.K2_GetActorLocation` _array_element_2) (`local.SumOfGridLocations`)))))
  (bind _output_get_2 (set `local.MiddleLocation` (/ _output_get (`KismetArrayLibrary.Array_Length` _filtrered_grid))))
  ;[1 1 1] Spawn First Actor (Bottom)
  (bind _returnvalue_2 (`|SpawnActorFromClass` Item (`KismetMathLibrary.MakeTransform` _output_get_2 (`KismetMathLibrary.ComposeRotators` (`Actor.K2_GetActorRotation` ActorAttached) Rotation)) "Undefined" "MultiplyWithRoot" null null))
  (`/Engine/EditorBlueprintResources/StandardMacros.IsValid` _returnvalue_2
    (:`Is Valid`
      (`Actor.K2_SetActorLocation` _returnvalue_2 (+ _output_get_2 (`KismetMathLibrary.MakeVector` 0.0 0.0 (.z (`.BoxExtent` (`KismetSystemLibrary.GetComponentBounds` (`/Game/Blueprints/ItemInteractables/BP_A_ItemInteractable.StaticMesh` _returnvalue_2)))))) false false)
      (set `/Game/Blueprints/ItemInteractables/BP_A_ItemInteractable.GridUsed` (`local.Filtrered Grid`) _returnvalue_2)
      (set `/Game/Blueprints/ItemInteractables/BP_A_ItemInteractable.canBeDragged` true _returnvalue_2)
      (set `/Game/Blueprints/ItemInteractables/BP_A_ItemInteractable.StackOwner` _returnvalue_2 _returnvalue_2)
      (`Actor.K2_AttachToActor` _returnvalue_2 (`|GetArrayItem` (`local.Filtrered Grid`)) "None" "KeepWorld" "KeepWorld" "KeepWorld" true)
      (`KismetArrayLibrary.Array_Add` (`local.Items`) _returnvalue_2)
      (`KismetArrayLibrary.Array_Add` InItems _returnvalue_2)
      ;[1 1 1] Spawn next actors (Stacking)
      (if (> NumberOfItems 1)
        (for _ (range (+ (- NumberOfItems 2) 1))
          (bind _returnvalue_3 (`|SpawnActorFromClass` Item (`KismetMathLibrary.MakeTransform` _returnvalue (`SceneComponent.K2_GetComponentRotation` _arrow)) "Undefined" "MultiplyWithRoot" null null))
          (`Actor.K2_SetActorLocation` _returnvalue_3 _returnvalue false false)
          (set `/Game/Blueprints/ItemInteractables/BP_A_ItemInteractable.GridUsed` (`local.Filtrered Grid`) _returnvalue_3)
          (set `/Game/Blueprints/ItemInteractables/BP_A_ItemInteractable.canBeDragged` true _returnvalue_3)
          (`Actor.K2_AttachToActor` _returnvalue_3 (`|GetArrayItem` (`local.Filtrered Grid`)) "None" "KeepWorld" "KeepWorld" "KeepWorld" true)
          (set `/Game/Blueprints/ItemInteractables/BP_A_ItemInteractable.StackOwner` _returnvalue_2 _returnvalue_3)
          (`KismetArrayLibrary.Array_Add` (`local.Items`) _returnvalue_3)
          (`KismetArrayLibrary.Array_Add` (`/Game/Blueprints/ItemInteractables/BP_A_ItemInteractable.ItemStack` _returnvalue_2) _returnvalue_3)
          (`KismetArrayLibrary.Array_Add` InItems _returnvalue_3)))
      (for _array_element_3 (`local.Items`)
        (`/Engine/EditorBlueprintResources/StandardMacros.IsValid` _array_element_3
          (:`Is Valid`
            (`PrimitiveComponent.SetCollisionEnabled` (`/Game/Blueprints/ItemInteractables/BP_A_ItemInteractable.Collision` _array_element_3) "NoCollision"))))
      (for _array_element_4 (`local.Filtrered Grid`)
        (set `/Game/Blueprints/Box/Grids/BP_A_Grid.isOccupied` true _array_element_4)
        (set `/Game/Blueprints/Box/Grids/BP_A_Grid.ItemOccupied` _returnvalue_2 _array_element_4)
        (`PrimitiveComponent.SetMaterial` (`/Game/Blueprints/Box/Grids/BP_A_Grid.Grid` _array_element_4) 0 "/Game/Textures/GridMaterial_InstRed.GridMaterial_InstRed")))))