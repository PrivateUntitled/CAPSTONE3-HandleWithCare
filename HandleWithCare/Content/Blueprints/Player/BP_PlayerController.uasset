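; Player controller for a house packing and unpacking game, handling mouse mode and hotkeys that appear to be largely for testing.
; Tick locks the cursor to screen center while roaming, and SetMouse switches cursor visibility and input mode.
; Keys call game mode hooks before changing levels, respawn saved packages from the game instance, and pause to score item placement on a results screen or dismiss it.
; An older package-saving routine remains disconnected.
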(event `self.ReceiveTick`
  (params (DeltaSeconds :type "Float (single-precision)"))
  (bind (_returnvalue_x _returnvalue_y) (`KismetMathLibrary.BreakVector2D` (`WidgetLayoutLibrary.GetViewportSize`)))
  (if (`self.Roaming`)
    (`self.SetMouseLocation` (`KismetMathLibrary.FTrunc` (/ _returnvalue_x 2.0)) (`KismetMathLibrary.FTrunc` (/ _returnvalue_y 2.0)))))

(event `self.ReceiveBeginPlay`
  (bind _asbp_gm_main (cast `/Game/Blueprints/GameModes/BP_GM_Main` (`GameplayStatics.GetGameMode`)))
  (set `self.As BP GM Main` _asbp_gm_main))

(event `Key|SpaceBar`
  (params (Key :type "Key Structure"))
  (:`Pressed`
    (`/Game/Blueprints/GameModes/BP_GM_Main.OnExitHouse` (`self.As BP GM Main`))
    (`KismetSystemLibrary.PrintString` "Unpacking House")
    (`GameplayStatics.OpenLevelBySoftObjectPtr` "/Game/GameInstance/GameInstanceTest2.GameInstanceTest2")))

(event `Key|B`
  (params (Key :type "Key Structure"))
  (:`Pressed`
    (`/Game/Blueprints/GameModes/BP_GM_Main.OnNextLevel` (`self.As BP GM Main`))
    (`KismetSystemLibrary.PrintString` "New House")
    (`GameplayStatics.OpenLevelBySoftObjectPtr` "/Game/GameInstance/GameInstanceTest.GameInstanceTest")))

(event `Key|N`
  (params (Key :type "Key Structure"))
  (:`Pressed`
    ;[1 1 1] Spawn testing
    (bind _asbp_game_instance (cast `/Game/GameInstance/BP_GameInstance` (`GameplayStatics.GetGameInstance`)))
    (`/Game/Blueprints/Player/BP_AC_PopulateItems.Populate Saved Items` (`self.BP_AC_PopulateItems`) (`/Game/GameInstance/BP_GameInstance.Packages` _asbp_game_instance) (`self.NewVar`) (`self.NewVar_0`))))

(event `Key|H`
  (params (Key :type "Key Structure"))
  (bind _as_bp_gm_main (`self.As BP GM Main`))
  (bind _resultscreenwidget (`/Game/Blueprints/GameModes/BP_GM_Main.ResultScreenWidget` (`self.As BP GM Main`)))
  (:`Pressed`
    (`GameplayStatics.SetGamePaused` true)
    (set `self.Roaming` false)
    (set `self.bShowMouseCursor` true)
    (`/Game/Blueprints/GameModes/BP_GM_Main.CheckItemPlacements` _as_bp_gm_main)
    (`KismetSystemLibrary.PrintString` (`KismetTextLibrary.Conv_TextToString` (`|FormatText` "Correct Items: {int} \nWrong items: {int2}" (`KismetArrayLibrary.Array_Length` (`/Game/Blueprints/GameModes/BP_GM_Main.CorrectItems` _as_bp_gm_main)) (`KismetArrayLibrary.Array_Length` (`/Game/Blueprints/GameModes/BP_GM_Main.WrongItems` _as_bp_gm_main)))))
    (`UserWidget.AddToViewport` _resultscreenwidget 0)
    (for _array_element (`/Game/Blueprints/Widgets/WB_ResultScreen.Stars` _resultscreenwidget)
      (`KismetSystemLibrary.PrintString` (`KismetSystemLibrary.GetDisplayName` _array_element)))))

(event `Key|J`
  (params (Key :type "Key Structure"))
  (bind _resultscreenwidget (`/Game/Blueprints/GameModes/BP_GM_Main.ResultScreenWidget` (`self.As BP GM Main`)))
  (:`Pressed`
    (`/Game/Blueprints/Widgets/WB_ResultScreen.RemoveReviews` _resultscreenwidget)
    (`Widget.RemoveFromParent` _resultscreenwidget)))

(fn `SetMouse`
  (params (Roaming :type Boolean) (ShowMouse :type Boolean))
  (set `self.Roaming` Roaming)
  (set `self.bShowMouseCursor` ShowMouse)
  (if ShowMouse
    (`WidgetBlueprintLibrary.SetInputMode_GameAndUIEx` self null "DoNotLock" false)
    (else
      (`WidgetBlueprintLibrary.SetInputMode_GameOnly` self))))

(fn `UserConstructionScript`)