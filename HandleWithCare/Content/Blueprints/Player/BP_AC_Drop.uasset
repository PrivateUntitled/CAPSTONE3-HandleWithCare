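; BP_AC_Drop handles dropping carried items from the Items array of the player's BP_ThirdPersonCharacter.
; Right mouse, when the player is not interacting, detaches the last item, resets its rotation, re-enables collision and physics, then recalculates carried weight.
; DropHoveredItem releases a specified item the same way, without the rotation reset or weight update, and moves it to the current furniture's DropLocation if one is valid.
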(event `self.ReceiveBeginPlay`
  (bind _asbp_third_person_character (cast `/Game/ThirdPerson/Blueprints/BP_ThirdPersonCharacter` (`GameplayStatics.GetPlayerPawn` 0)))
  (set `self.As BP Third Person Character` _asbp_third_person_character))

(event `Key|RightMouseButton`
  (params (Key :type "Key Structure"))
  (:`Pressed`
    (if (not (`/Game/ThirdPerson/Blueprints/BP_ThirdPersonCharacter.IsInteracting` (`self.As BP Third Person Character`)))
      (`self.Dropitem`))))

(event `Dropitem`
  (bind _items (`/Game/ThirdPerson/Blueprints/BP_ThirdPersonCharacter.Items` (`self.As BP Third Person Character`)))
  (bind _returnvalue (`KismetArrayLibrary.Array_LastIndex` _items))
  (bind _output (`|GetArrayItem` _items _returnvalue))
  (bind _collision (`/Game/Blueprints/ItemInteractables/BP_A_ItemInteractable.Collision` _output))
  (if (`KismetArrayLibrary.Array_IsValidIndex` (`/Game/ThirdPerson/Blueprints/BP_ThirdPersonCharacter.Items` (`self.As BP Third Person Character`)))
    (set `/Game/Blueprints/ItemInteractables/BP_A_ItemInteractable.canBeDragged` false _output)
    (`Actor.K2_SetActorRotation` :`self` _output)
    (`Actor.K2_DetachFromActor` _output "KeepWorld" "KeepWorld" "KeepWorld")
    (`PrimitiveComponent.SetCollisionEnabled` _collision "QueryAndPhysics")
    (`PrimitiveComponent.SetCollisionResponseToChannel` _collision "ECC_Visibility" "ECR_Block")
    (`PrimitiveComponent.SetSimulatePhysics` _collision true)
    (`KismetArrayLibrary.Array_Remove` _items _returnvalue)
    (`KismetSystemLibrary.PrintString` "DRopped")
    (`/Game/ThirdPerson/Blueprints/BP_ThirdPersonCharacter.CalculateWeight` (`self.As BP Third Person Character`))))

(event `DropHoveredItem`
  (params (HoveredItem :type "/Game/Blueprints/ItemInteractables/BP_A_ItemInteractable Object Reference"))
  (bind _collision (`/Game/Blueprints/ItemInteractables/BP_A_ItemInteractable.Collision` HoveredItem))
  (bind _currentfurniture (`/Game/ThirdPerson/Blueprints/BP_ThirdPersonCharacter.CurrentFurniture` (`self.As BP Third Person Character`)))
  (`Actor.K2_DetachFromActor` HoveredItem "KeepWorld" "KeepWorld" "KeepWorld")
  (`PrimitiveComponent.SetCollisionEnabled` _collision "QueryAndPhysics")
  (`PrimitiveComponent.SetCollisionResponseToChannel` _collision "ECC_Visibility" "ECR_Block")
  (`PrimitiveComponent.SetSimulatePhysics` _collision true)
  (`KismetArrayLibrary.Array_RemoveItem` (`/Game/ThirdPerson/Blueprints/BP_ThirdPersonCharacter.Items` (`self.As BP Third Person Character`)) HoveredItem)
  (`/Engine/EditorBlueprintResources/StandardMacros.IsValid` _currentfurniture
    (:`Is Valid`
      (`Actor.K2_SetActorLocation` HoveredItem (`SceneComponent.K2_GetComponentLocation` (`/Game/Blueprints/Furniture/BP_A_Furniture.DropLocation` _currentfurniture)) false false))))