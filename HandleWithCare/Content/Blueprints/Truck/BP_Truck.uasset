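; BP_Truck is an interactable truck that spawns physics-simulated packages at a drop-off area.
; On BeginPlay it recreates packages saved in the GameInstance and attaches their stored items inside.
; Cursor hover enables E input, which spawns an empty package up to a maximum count, unless the player's first item is openable.
; SpawnPackage picks a random point in a box component, raised slightly so packages drop to the ground.
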(event `self.ReceiveBeginPlay`
  (bind _asbp_third_person_character (cast `/Game/ThirdPerson/Blueprints/BP_ThirdPersonCharacter` (`GameplayStatics.GetPlayerPawn` 0)))
  (set `self.As BP Third Person Character` _asbp_third_person_character)
  (bind _asbp_gm_main (cast `/Game/Blueprints/GameModes/BP_GM_Main` (`GameplayStatics.GetGameMode`)))
  (set `self.As BP GM Main` _asbp_gm_main)
  (bind _asbp_game_instance (cast `/Game/GameInstance/BP_GameInstance` (`GameplayStatics.GetGameInstance`)))
  (set `self.As BP Game Instance` _asbp_game_instance)
  ;[0.4549 0.2588 0.7412] Check if max spawn is reached (for 0 Max Spawn Package)
  (set `self.CanSpawnPackages?` (< (`self.SpawnedPackages`) (`self.MaxSpawnPackageAmount`)))
  ;[0.4549 0.2588 0.7412] Spawn New Boxes
  ;;[0.7647 0.7647 0.7647] Spawn Package
  (for _array_element (`/Game/GameInstance/BP_GameInstance.Packages` (`self.As BP Game Instance`))
    (bind ((`ClassType_29_DED2E0094CE7CE81402D5F857B8E19EF` _classtype) (`ItemStruct_27_FD7B7C76463B1372BA6C239951008261` _itemstruct)) (break `/Game/Blueprints/Structure/PackageStruct` _array_element))
    (bind _spawnedpackage (`self.Spawn Package` _classtype))
    ;;[0.7647 0.7647 0.7647] Spawn Items of Box
    (for _array_element_2 _itemstruct
      (bind _returnvalue (`|SpawnActorFromClass` (break `/Game/Blueprints/Structure/ItemStruct` _array_element_2) (`KismetMathLibrary.MakeTransform` (`.Location_6_E6A949BB445CB969F790878C051740C6` (break `/Game/Blueprints/Structure/ItemStruct` _array_element_2)) (`.Rotation_9_F1B159DE4DBA65746B89F99085B07607` (break `/Game/Blueprints/Structure/ItemStruct` _array_element_2))) "Undefined" "MultiplyWithRoot" null null))
      (`KismetArrayLibrary.Array_AddUnique` (`/Game/Blueprints/Box/BP_A_Package.InBox` _spawnedpackage) _returnvalue)
      (`self.K2_AttachToActor` _returnvalue _spawnedpackage "None" "KeepRelative" "KeepRelative" "KeepRelative" true))))

(event `Key|E`
  (params (Key :type "Key Structure"))
  (bind _as_bp_third_person_character (`self.As BP Third Person Character`))
  ;[0.4549 0.2588 0.7412] Interact with Truck (Spawning Empty Boxes)
  (:`Pressed`
    (`/Engine/EditorBlueprintResources/StandardMacros.IsValid` _as_bp_third_person_character
      (:`Is Valid`
        (if (and (`self.CanSpawnPackages?`) (not (`KismetSystemLibrary.DoesImplementInterface` (`|GetArrayItem` (`/Game/ThirdPerson/Blueprints/BP_ThirdPersonCharacter.Items` _as_bp_third_person_character)) "/Game/Blueprints/ItemInteractables/BlueprintInterface/BI_Openable.BI_Openable_C")))
          ;;[0.7656 0.7656 0.7656] Spawn Empty Package
          (bind _spawnedpackage (`self.Spawn Package` (`self.PackageClass`)))
          ;;[0.7647 0.7647 0.7647] Disable Spawn if max amt has been reached
          (`/Engine/EditorBlueprintResources/StandardMacros.IncrementInt` (`self.SpawnedPackages`)
            (:`  `
              (set `self.CanSpawnPackages?` (< (`self.SpawnedPackages`) (`self.MaxSpawnPackageAmount`))))))))))

(event `self.Box.OnBeginCursorOver`
  (params (TouchedComponent :type "PrimitiveComponent Object Reference"))
  (bind _as_bp_third_person_character (`self.As BP Third Person Character`))
  ;[0.4554 0.2597 0.7396] Enable Interact (E) when cursor on the truck
  (`/Engine/EditorBlueprintResources/StandardMacros.IsValid` (`self.As BP Third Person Character`)
    (:`Is Valid`
      (if (not (`/Game/ThirdPerson/Blueprints/BP_ThirdPersonCharacter.IsInteracting` (`self.As BP Third Person Character`)))
        (set `/Game/ThirdPerson/Blueprints/BP_ThirdPersonCharacter.HasHoveredItem` true _as_bp_third_person_character)
        (`self.EnableInput` (`/Game/ThirdPerson/Blueprints/BP_ThirdPersonCharacter.As BP Player Controller` _as_bp_third_person_character))))))

(event `self.Box.OnEndCursorOver`
  (params (TouchedComponent :type "PrimitiveComponent Object Reference"))
  (bind _as_bp_third_person_character (`self.As BP Third Person Character`))
  ;[0.4554 0.2597 0.7396] Disable Interact (E) when cursor off the truck
  (`/Engine/EditorBlueprintResources/StandardMacros.IsValid` (`self.As BP Third Person Character`)
    (:`Is Valid`
      (if (not (`/Game/ThirdPerson/Blueprints/BP_ThirdPersonCharacter.IsInteracting` (`self.As BP Third Person Character`)))
        (set `/Game/ThirdPerson/Blueprints/BP_ThirdPersonCharacter.HasHoveredItem` false _as_bp_third_person_character)
        (`self.DisableInput` (`/Game/ThirdPerson/Blueprints/BP_ThirdPersonCharacter.As BP Player Controller` _as_bp_third_person_character))))))

(fn `Spawn Package`
  (params (PackageToSpawn :type "/Game/Blueprints/Box/BP_A_Package Class Reference"))
  (returns (SpawnedPackage :type "/Game/Blueprints/Box/BP_A_Package Object Reference"))
  (bind _box1 (`self.Box1`))
  (bind (_returnvalue_x _returnvalue_y _returnvalue_z) (`KismetMathLibrary.BreakVector` (`KismetMathLibrary.RandomPointInBoundingBox` (`SceneComponent.K2_GetComponentLocation` _box1) (`BoxComponent.BoxExtent` _box1))))
  (bind _returnvalue (`|SpawnActorFromClass` PackageToSpawn (`KismetMathLibrary.Conv_VectorToTransform` (`KismetMathLibrary.MakeVector` _returnvalue_x _returnvalue_y (+ _returnvalue_z 100.0))) "Undefined" "MultiplyWithRoot" null null))
  (bind _collision (`/Game/Blueprints/ItemInteractables/BP_A_ItemInteractable.Collision` _returnvalue))
  ;[0.7647 0.7647 0.7647] Drop Box to the Ground (Physics)
  (`PrimitiveComponent.SetCollisionEnabled` _collision "QueryAndPhysics")
  (`PrimitiveComponent.SetCollisionResponseToChannel` _collision "ECC_Visibility" "ECR_Block")
  (`PrimitiveComponent.SetSimulatePhysics` _collision true)
  (return _returnvalue))

(fn `UserConstructionScript`)